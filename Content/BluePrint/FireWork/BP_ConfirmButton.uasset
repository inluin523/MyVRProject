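; VR confirm button for a hot-work permit training scenario, pressed through the motion controller's Pickup event.
; Three flags select the stage (approval, permit issuing with hazard notice, final confirmation), each animating the button with paired timelines.
; Stages swap TV screen and button-state actors through timed delays, with the last logging a score of 100.
; CheckWorkBefore tests four FireGameMode safety flags, then advances the screens or reveals failure actors.
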(event Custom|CheckWorkBefore
  (bind _asfire_game_mode (Utilities|Casting|CastToFireGameMode (Game|GetGameMode)))
  (if (Math|Boolean|ANDBoolean (Variables|/Game/BluePrint/FireGameMode.FireGameMode_C|GetIsSecurityCorrect _asfire_game_mode) (Variables|/Game/BluePrint/FireGameMode.FireGameMode_C|GetIsCloseTap _asfire_game_mode) (Variables|/Game/BluePrint/FireGameMode.FireGameMode_C|GetIsDetectGas _asfire_game_mode) (Variables|/Game/BluePrint/FireGameMode.FireGameMode_C|GetIsClearGabarage _asfire_game_mode))
    (Rendering|SetActorHiddenInGame (Variables|Default|GetconfirmBT6) true)
    (Rendering|SetActorHiddenInGame (Variables|Default|GetconfirmBT2) false)
    (Rendering|SetActorHiddenInGame (Variables|Default|Gettvuiactor5) true)
    (Rendering|SetActorHiddenInGame (Variables|Default|Gettvuiactor6) false)
    (bind _asfire_game_mode_2 (Utilities|Casting|CastToFireGameMode (Game|GetGameMode)))
    (Variables|/Game/BluePrint/FireGameMode.FireGameMode_C|SetIssecondFY _asfire_game_mode_2 true)
    (else
      (Rendering|SetActorHiddenInGame (Variables|Default|Getshibaitishi2222) false)
      (Rendering|SetActorHiddenInGame (Variables|Default|Getshibaiscore) false)
      (Rendering|SetActorHiddenInGame (Variables|Default|GetZYQBZYLACTOR) false))))

(event EventPickup
  (params (AttachTo :type Scene%20Component%20Object%20Reference) (CharacterType :type EcharacterType%20Enum :default "NewEnumerator0"))
  (bind _confirmbt8 (Variables|Default|GetconfirmBT8))
  (bind _tvuiactor12 (Variables|Default|Gettvuiactor12))
  (bind _tvuiactor3 (Variables|Default|Gettvuiactor3))
  (bind _confirmbt7 (Variables|Default|GetconfirmBT7))
  (bind _tvuiactor8 (Variables|Default|Gettvuiactor8))
  (bind _confirmbt9 (Variables|Default|GetconfirmBT9))
  ;[1 1 1] 点击按钮审批成功
  (if (Variables|Default|GetIsBeforeWork)
    (if true
      ;[1 1 1] 按钮伸缩
      (bind _offset (Timeline|时间轴_0 Play)
        (:Update
          (Transformation|SetActorLocation (Math|Vector|MakeVector _offset -9298.837891 130.068115) false false))
        (:Finished
          (bind _offset_2 (Timeline|时间轴_1 PlayFromStart)
            (:Update
              (Transformation|SetActorLocation (Math|Vector|MakeVector _offset_2 -9298.837891 130.068115) false false)
              (Variables|Default|SetIsBeforeWork false)
              (Rendering|SetActorHiddenInGame (Variables|Default|GetconfirmBT1) true)
              (Rendering|SetActorHiddenInGame _confirmbt7 false)
              (Rendering|SetActorHiddenInGame (Variables|Default|Gettvuiactor2) true)
              (Rendering|SetActorHiddenInGame _tvuiactor3 false)
              (Utilities|FlowControl|Delay 5.0)
              (Rendering|SetActorHiddenInGame _confirmbt7 true)
              (Rendering|SetActorHiddenInGame (Variables|Default|GetconfirmBT5) false)
              (Rendering|SetActorHiddenInGame _tvuiactor3 true)
              (Rendering|SetActorHiddenInGame (Variables|Default|Gettvuiactor4) false)
              (Rendering|SetActorHiddenInGame (Variables|Default|GetFanYe) false))))))
    (else
      ;[1 1 1] 点击按钮签发作业许可证并显示危险告知
      (if (Variables|Default|GetisCanQianFa)
        (if true
          (bind _offset_3 (Timeline|时间轴_2 Play)
            (:Update
              (Transformation|SetActorLocation (Math|Vector|MakeVector _offset_3 -9298.837891 130.068115) false false))
            (:Finished
              (bind _offset_4 (Timeline|时间轴_3 PlayFromStart)
                (:Update
                  (Transformation|SetActorLocation (Math|Vector|MakeVector _offset_4 -9298.837891 130.068115) false false)
                  (Variables|Default|SetisCanQianFa false)
                  (Rendering|SetActorHiddenInGame (Variables|Default|Gettvuiactor7) true)
                  (Rendering|SetActorHiddenInGame _tvuiactor8 false)
                  (Rendering|SetActorHiddenInGame (Variables|Default|GetconfirmBT2) true)
                  (Rendering|SetActorHiddenInGame _confirmbt9 false)
                  (Utilities|FlowControl|Delay 6.0)
                  (Rendering|SetActorHiddenInGame _confirmbt9 true)
                  (Rendering|SetActorHiddenInGame (Variables|Default|GetconfirmBT3) false)
                  (Rendering|SetActorHiddenInGame _tvuiactor8 true)
                  (Rendering|SetActorHiddenInGame (Variables|Default|Gettvuiactor9) false)
                  (bind _asfire_game_mode (Utilities|Casting|CastToFireGameMode (Game|GetGameMode)))
                  (Variables|/Game/BluePrint/FireGameMode.FireGameMode_C|SetIsThirdFY _asfire_game_mode true)
                  (Rendering|SetActorHiddenInGame (Variables|Default|GetdhzyCameraact1) false))))))
        (elif (Variables|Default|GetisCanQueRen)
          (bind _offset_5 (Timeline|时间轴_4 Play)
            (:Update
              (Transformation|SetActorLocation (Math|Vector|MakeVector _offset_5 -9298.837891 130.068115) false false))
            (:Finished
              (bind _offset_6 (Timeline|时间轴_5 PlayFromStart)
                (:Update
                  (Transformation|SetActorLocation (Math|Vector|MakeVector _offset_6 -9298.837891 130.068115) false false)
                  (Variables|Default|SetisCanQueRen false)
                  (Rendering|SetActorHiddenInGame (Variables|Default|Gettvuiactor8) true)
                  (Rendering|SetActorHiddenInGame (Variables|Default|Gettvuicator11) false)
                  (Rendering|SetActorHiddenInGame (Variables|Default|GetconfirmBT4) true)
                  (Rendering|SetActorHiddenInGame _confirmbt8 false)
                  (Utilities|FlowControl|Delay 5.0)
                  (Rendering|SetActorHiddenInGame _confirmbt8 true)
                  (Rendering|SetActorHiddenInGame _tvuiactor12 false)
                  (Utilities|FlowControl|Delay 6.0)
                  (Rendering|SetActorHiddenInGame _tvuiactor12 true)
                  (Rendering|SetActorHiddenInGame (Variables|Default|Getdhzydengji) false)
                  (Development|PrintString "scorescore:100" false))))))))))

(event EventDrop)

(fn ConstructionScript)

(fn GetText
  (params (NewParam :type Boolean))
  (if NewParam
    (return "是")
    (else
      (return "否"))))