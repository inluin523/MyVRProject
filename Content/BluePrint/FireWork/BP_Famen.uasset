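; BP_Famen is a valve actor in a fire game that checks whether the player has completed a valve-closing procedure.
; Box overlaps record the blind plate, its sign and the wrench; placing the sign also swaps it for a preset actor and triggers the check.
; The check requires all three plus tap rotation, then marks the tap closed in FireGameMode, hides a widget and calls Fmss.
; Otherwise it reveals failure actors.
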(event OnComponentBeginOverlap(Box)
  (params (OverlappedComponent :type Primitive%20Component%20Object%20Reference) (OtherActor :type Actor%20Object%20Reference) (OtherComp :type Primitive%20Component%20Object%20Reference) (OtherBodyIndex :type Integer) (bFromSweep :type Boolean) (SweepResult :type Hit%20Result%20Structure%20%28by%20ref%29))
  (bind _asfire_game_mode (Utilities|Casting|CastToFireGameMode (Game|GetGameMode)))
  (if (not (Variables|/Game/BluePrint/FireGameMode.FireGameMode_C|GetIsCloseTap _asfire_game_mode))
    (bind _asmang_ban_biao_zhi_actor (Utilities|Casting|CastToMangBanBiaoZhiActor OtherActor)
      (:then
        (Actor|DestroyActor _asmang_ban_biao_zhi_actor)
        (Rendering|SetActorHiddenInGame (Variables|Default|GetMangBanBiaoZhiActorPos) false)
        (Variables|Default|SetIsBiaozhiCorrect true)
        (if true
          (CallFunction|Jiance)))
      (:CastFailed
        (Utilities|Casting|CastToMangBan OtherActor
          (:then
            (Variables|Default|SetIsMangBanCorrect true))
          (:CastFailed
            (Utilities|Casting|CastTobanShouActor OtherActor)
            (Variables|Default|SetIsBanShou true)))))))

(event Custom|jiance
  (if (Math|Boolean|ANDBoolean (Variables|Default|GetIsMangBanCorrect) (Variables|Default|GetIsBiaozhiCorrect) (Variables|/Game/ceTest/Tap.Tap_C|GetisXuanZhuan (Variables|Default|GetISTapXuanZhuan)) (Variables|Default|GetIsBanShou))
    (bind _asfire_game_mode (Utilities|Casting|CastToFireGameMode (Game|GetGameMode)))
    (Variables|/Game/BluePrint/FireGameMode.FireGameMode_C|SetIsCloseTap _asfire_game_mode true)
    (Rendering|SetVisibility (Variables|Default|GetWidget) false false)
    (Default|Fmss (Variables|Default|Getfmss))
    (else
      (Rendering|SetActorHiddenInGame (Variables|Default|Getshibaiactor) false)
      (Rendering|SetActorHiddenInGame (Variables|Default|Getshibaichengji) false)
      (Rendering|SetActorHiddenInGame (Variables|Default|Getfmczywactor111) false))))

(event EventBeginPlay)

(event Collision|EventActorBeginOverlap
  (params (OtherActor :type Actor%20Object%20Reference)))

(event EventTick
  (params (DeltaSeconds :type Float%20%28single-precision%29)))

(fn ConstructionScript)