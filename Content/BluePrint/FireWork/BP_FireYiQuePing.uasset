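; BP_FireYiQuePing is a networked VR pickup prop, apparently an acetylene cylinder in the FireWork content.
; Pickup attaches it to the motion controller and starts a 0.05s timer sending hand-based transforms through MyPlayerController, with roll adjusted by hand scale sign.
; Drop stops the timer, detaches it, then snaps it to a vertical WorldStatic trace hit.
; OnRep_pos applies replicated transforms; both Pickup and Drop set IsPickUp false.
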(event Custom|GetXifu
  (bind _hightpos (Variables|Default|GetHightpos))
  (bind _returnvalue (Transformation|GetWorldLocation _hightpos))
  (bind (_x _y _z) (Math|Vector|BreakVector _returnvalue))
  (bind _outhit (Collision|LineTraceForObjects (Math|Vector|MakeVector _x _y (+ _z 3e+02)) (Math|Vector|MakeVector _x _y (+ _z -3e+02)) (Utilities|Array|MakeArray "ObjectTypeQuery1") true 0 "None"))
  (bind _asmy_player_controller (Utilities|Casting|CastToMyPlayerController (Game|GetPlayerController 0)))
  (Default|UpdatePickUpPosC _asmy_player_controller self (Math|Transform|MakeTransform (Math|Vector|MakeVector (.X (Math|Vector|BreakVector (.Location (Collision|BreakHitResult _outhit)))) (.Y (Math|Vector|BreakVector (.Location (Collision|BreakHitResult _outhit)))) (+ (.Z (Math|Vector|BreakVector (.Location (Collision|BreakHitResult _outhit)))) 4.0)) (Math|Rotator|MakeRotator 0.0 0.0 (.yaw (Transformation|GetWorldRotation (Variables|Debug|GetStaticMeshComponent)))) (Transformation|GetWorldScale (Variables|Default|GetHightpos)))))

(event Custom|UpdatePos_C
  (bind _self self)
  (bind _staticmesh (Variables|Default|GetStaticMesh))
  (bind _hand (Variables|Default|GetHand))
  (bind _scene (Variables|Default|GetScene))
  (bind _returnvalue (Transformation|GetWorldTransform _hand))
  (bind _returnvalue_2 (Transformation|GetWorldLocation _staticmesh))
  (bind _returnvalue_3 (Transformation|GetWorldLocation _scene))
  (bind _returnvalue_4 (- _returnvalue_2 _returnvalue_3))
  (bind (_roll _pitch _yaw) (Math|Rotator|BreakRotator (.rotation _returnvalue)))
  (bind _returnvalue_5 (+ (.location _returnvalue) _returnvalue_4))
  (bind _asmy_player_controller (Utilities|Casting|CastToMyPlayerController (Game|GetPlayerController 0)))
  (if (< (.Y (Math|Vector|BreakVector (.scale _returnvalue))) 0.0)
    (Default|UpdatePickUpPosC _asmy_player_controller _self (Math|Transform|MakeTransform _returnvalue_5 (Math|Rotator|MakeRotator (+ _roll 9e+01) _pitch _yaw) (Transformation|GetWorldScale (Variables|Default|GetScene))))
    (else
      (Default|UpdatePickUpPosC _asmy_player_controller _self (Math|Transform|MakeTransform _returnvalue_5 (Math|Rotator|MakeRotator (- _roll 2.8) _pitch _yaw) (Transformation|GetWorldScale (Variables|Default|GetScene)))))))

(event Custom|SetPickUp_S
  (params (IsPickUp :type Boolean))
  ;[1 1 1] 设置物体被抓
  (Variables|Default|SetIsPickUp IsPickUp))

(event EventPickup
  (params (AttachTo :type Scene%20Component%20Object%20Reference) (CharacterType :type EcharacterType%20Enum :default "NewEnumerator0"))
  (Variables|Default|SetHand AttachTo)
  (Utilities|FlowControl|Sequence
    (:then_0
      (CallFunction|SetPickUpS false))
    (:then_1
      (Transformation|AttachComponentToComponent (VehicleSound|GetRootComponent) AttachTo "None" "KeepWorld" "KeepWorld" "KeepWorld" false))
    (:then_2
      ;[1 1 1] 心跳同步
      (Utilities|Time|SetTimerbyFunctionName 0 "UpdatePos" 0.05 true))))

(event EventDrop
  (Utilities|FlowControl|Sequence
    (:then_0
      ;[1 1 1] 设置灭火器不被抓
      (CallFunction|SetPickUpS false))
    (:then_1
      ;[1 1 1] 取消心跳同步
      (Utilities|Time|ClearTimerbyFunctionName 0 "UpdatePos"))
    (:then_2
      (Transformation|DetachFromActor "KeepWorld" "KeepWorld" "KeepWorld"))
    (:then_3
      (CallFunction|GetXifu))))

(fn ConstructionScript)

(fn OnRepPos
  (bind _pos (Variables|Default|Getpos))
  (if (Math|Vector|NotEqual(Vector) (.Location (Math|Transform|BreakTransform _pos)) "0, 0, 0" 0.1)
    (Transformation|SetWorldTransform (Variables|Debug|GetStaticMeshComponent) _pos false false)))

(fn UpdatePos
  (CallFunction|UpdatePosC))