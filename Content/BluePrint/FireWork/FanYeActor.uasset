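; Interactive FanYe actor in the FireWork sequence that slides along X when picked up, advancing up to three procedure stages.
; Pickup selects a stage from its first-pick flag or FireGameMode's second/third flags, then plays two chained timelines.
; Timeline updates clear the flag and swap TV screen and confirm-button visibility.
; Stage two enables ConfirmBT's QianFa; stage three spawns HanqiangActor and sets GameMode camera and after-work flags.
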(event EventPickup
  (params (AttachTo :type Scene%20Component%20Object%20Reference) (CharacterType :type EcharacterType%20Enum :default "NewEnumerator0"))
  (if (Variables|Default|GetFirestPick)
    (bind _offset (Timeline|时间轴_0 Play)
      (:Update
        (Transformation|SetActorLocation (Math|Vector|MakeVector _offset -8901.201172 85.030334) false false)
        (Variables|Default|SetFirestPick false)
        (Rendering|SetActorHiddenInGame (Variables|Default|Gettuuiactor4) true)
        (Rendering|SetActorHiddenInGame (Variables|Default|Gettvuiactor5) false)
        (Utilities|FlowControl|Delay 8.0)
        (Rendering|SetActorHiddenInGame (Variables|Default|GetconfirmBT5) true)
        (Rendering|SetActorHiddenInGame (Variables|Default|GetconfirmBT6) false))
      (:Finished
        (bind _offset_2 (Timeline|时间轴_1 PlayFromStart)
          (:Update
            (Transformation|SetActorLocation (Math|Vector|MakeVector _offset_2 -8901.201172 85.030334) false false)))))
    (else
      (bind _asfire_game_mode (Utilities|Casting|CastToFireGameMode (Game|GetGameMode)))
      (if (Variables|/Game/BluePrint/FireGameMode.FireGameMode_C|GetIssecondFY _asfire_game_mode)
        (bind _offset_3 (Timeline|时间轴_2 Play)
          (:Update
            (Transformation|SetActorLocation (Math|Vector|MakeVector _offset_3 -8901.201172 85.030334) false false)
            (Variables|/Game/BluePrint/FireGameMode.FireGameMode_C|SetIssecondFY _asfire_game_mode false)
            (Rendering|SetActorHiddenInGame (Variables|Default|Gettvuiactor6) true)
            (Rendering|SetActorHiddenInGame (Variables|Default|Gettvuiactor7) false)
            (Variables|/Game/BluePrint/FireWork/BP_ConfirmButton.BP_ConfirmButton_C|SetisCanQianFa (Variables|Default|GetConfirmBT) true))
          (:Finished
            (bind _offset_4 (Timeline|时间轴_3 PlayFromStart)
              (:Update
                (Transformation|SetActorLocation (Math|Vector|MakeVector _offset_4 -8901.201172 85.030334) false false)))))
        (elif (Variables|/Game/BluePrint/FireGameMode.FireGameMode_C|GetIsThirdFY _asfire_game_mode)
          (bind _offset_5 (Timeline|时间轴_4 Play)
            (:Update
              (Transformation|SetActorLocation (Math|Vector|MakeVector _offset_5 -8901.201172 85.030334) false false))
            (:Finished
              (bind _offset_6 (Timeline|时间轴_5 PlayFromStart)
                (:Update
                  (Transformation|SetActorLocation (Math|Vector|MakeVector _offset_6 -8901.201172 85.030334) false false)
                  (Variables|/Game/BluePrint/FireGameMode.FireGameMode_C|SetIsThirdFY _asfire_game_mode false)
                  (Rendering|SetActorHiddenInGame (Variables|Default|Gettvuiactor9) true)
                  (Rendering|SetActorHiddenInGame (Variables|Default|Gettvuiactor10) false)
                  (Utilities|FlowControl|Delay 5.0)
                  (Rendering|SetActorHiddenInGame (Variables|Default|GetconfirmBT3) true)
                  (Rendering|SetActorHiddenInGame (Variables|Default|Getworkactor1) false)
                  (bind _asfire_game_mode_2 (Utilities|Casting|CastToFireGameMode (Game|GetGameMode)))
                  (Game|SpawnActorfromClass "/Game/ceTest/hanqiangActor.hanqiangActor_C" (Transformation|GetActorTransform (Variables|Default|Gethanqiang)) "Undefined" 0 0)
                  (Variables|/Game/BluePrint/FireGameMode.FireGameMode_C|SetIsCamera _asfire_game_mode_2 true)
                  (Variables|/Game/BluePrint/FireGameMode.FireGameMode_C|SetisAfterWork _asfire_game_mode_2 true))))))))))

(fn ConstructionScript)