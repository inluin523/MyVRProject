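; FirePipe is a pipe station in a hot-work exercise, driven by Box overlaps and FireGameMode flags.
; A motion controller with a visible gas detector fills in preset GasDetectionUI readings, sets IsDetectGas and hides the widget.
; With ISSTARTCAREMER set, a welding gun (hanqiangActor) triggers delayed BP_Fire spawns at FireExplodePos, sets IsDoWork and swaps work actors.
; Without that flag, any non-controller overlap reveals three hidden actors, apparently failure notices.
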(event OnComponentBeginOverlap(Box)
  (params (OverlappedComponent :type Primitive%20Component%20Object%20Reference) (OtherActor :type Actor%20Object%20Reference) (OtherComp :type Primitive%20Component%20Object%20Reference) (OtherBodyIndex :type Integer) (bFromSweep :type Boolean) (SweepResult :type Hit%20Result%20Structure%20%28by%20ref%29))
  (bind _asbp_motion_controller (Utilities|Casting|CastToBP_MotionController OtherActor)
    (:then
      (bind _asfire_game_mode (Utilities|Casting|CastToFireGameMode (Game|GetGameMode)))
      (if (not (Variables|/Game/BluePrint/FireGameMode.FireGameMode_C|GetIsDetectGas _asfire_game_mode))
        ;[1 1 1] 气体检测
        (if (Rendering|IsVisible (Variables|/Game/BluePrint/BP_MotionController.BP_MotionController_C|GetGasDetection _asbp_motion_controller))
          (bind _asgas_detection_ui (Utilities|Casting|CastToGasDetectionUI (UserInterface|GetUserWidgetObject (Variables|/Game/BluePrint/BP_MotionController.BP_MotionController_C|GetScreen _asbp_motion_controller))))
          (Variables|/Game/UI/FireWork/GasDetectionUI.GasDetectionUI_C|SetExplodeLimitText _asgas_detection_ui "5%")
          (Variables|/Game/UI/FireWork/GasDetectionUI.GasDetectionUI_C|SetGasDetectionText _asgas_detection_ui "0.3%")
          (Variables|/Game/BluePrint/FireGameMode.FireGameMode_C|SetIsDetectGas _asfire_game_mode true)
          (Rendering|SetVisibility (Variables|Default|GetWidget) false false))))
    (:CastFailed
      (bind _asfire_game_mode_2 (Utilities|Casting|CastToFireGameMode (Game|GetGameMode)))
      (if (Variables|/Game/BluePrint/FireGameMode.FireGameMode_C|GetISSTARTCAREMER _asfire_game_mode_2)
        (Utilities|Casting|CastTohanqiangActor OtherActor)
        ;[1 1 1] 进行作业
        (Utilities|FlowControl|Delay 5.0)
        (for _array_element (Variables|Default|GetFireExplodePos)
          (Game|SpawnActorfromClass "/Game/BluePrint/FireWork/BP_Fire.BP_Fire_C" (Transformation|GetActorTransform _array_element) "Undefined" 0 0)
          (bind _asfire_game_mode_3 (Utilities|Casting|CastToFireGameMode (Game|GetGameMode)))
          (Variables|/Game/BluePrint/FireGameMode.FireGameMode_C|SetisDoWork _asfire_game_mode_3 true)
          (Rendering|SetActorHiddenInGame (Variables|Default|Getworkactor1) true)
          (Rendering|SetActorHiddenInGame (Variables|Default|Getworkactor2) false))
        (else
          (Rendering|SetActorHiddenInGame (Variables|Default|Getdhzyscorewtg) false)
          (Rendering|SetActorHiddenInGame (Variables|Default|Getdhzywtg) false)
          (Rendering|SetActorHiddenInGame (Variables|Default|Getzyswksxjactor) false))))))

(fn ConstructionScript)