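; Placement target for the oxygen cylinder (YangQiPing) in what appears to be a fire-work safety exercise.
; When a BP_FireYangQiPing overlaps its Box, it destroys that actor and unhides its own Bottle and Gufing.
; It then branches on game mode: FireGameMode flags SecurityUIActor and calls BottleCorrect once, while BP_ZongHeGameMode flags ZhylBottuleactor and calls BottleUIyichu.
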(event OnComponentBeginOverlap(Box)
  (params (OverlappedComponent :type Primitive%20Component%20Object%20Reference) (OtherActor :type Actor%20Object%20Reference) (OtherComp :type Primitive%20Component%20Object%20Reference) (OtherBodyIndex :type Integer) (bFromSweep :type Boolean) (SweepResult :type Hit%20Result%20Structure%20%28by%20ref%29))
  (bind _zhylbottuleactor (Variables|Default|GetzhylBottuleactor))
  (bind _securityuiactor (Variables|Default|GetSecurityUIActor))
  (bind _asbp_fire_yang_qi_ping (Utilities|Casting|CastToBP_FireYangQiPing OtherActor))
  (Actor|DestroyActor _asbp_fire_yang_qi_ping)
  (Rendering|SetActorHiddenInGame (Variables|Default|Getbottle) false)
  (Rendering|SetActorHiddenInGame (Variables|Default|Getgufing) false)
  (Utilities|Casting|CastToFireGameMode (Game|GetGameMode)
    (:then
      (if (not (Variables|/Game/BluePrint/FireWork/SecurityUIIActor.SecurityUIIActor_C|GetIsYangQiPING _securityuiactor))
        (Variables|/Game/BluePrint/FireWork/SecurityUIIActor.SecurityUIIActor_C|SetIsYangQiPING _securityuiactor true)
        (Default|BottleCorrect _securityuiactor)))
    (:CastFailed
      (Utilities|Casting|CastToBP_ZongHeGameMode (Game|GetGameMode))
      (Variables|/Game/BluePrint/ZongHeYanLian/zhylBottleUIActor1.zhylBottleUIActor1_C|SetzhylIsYangQiPing _zhylbottuleactor true)
      (Default|BottleUIyichu _zhylbottuleactor))))

(event EventBeginPlay)

(event Collision|EventActorBeginOverlap
  (params (OtherActor :type Actor%20Object%20Reference)))

(event EventTick
  (params (DeltaSeconds :type Float%20%28single-precision%29)))

(fn ConstructionScript)