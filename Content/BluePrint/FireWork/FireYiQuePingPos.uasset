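; Placement spot for the acetylene cylinder (YiQuePing) in the fire-work scenario.
; When a BP_FireYiQuePing overlaps its Box, it destroys that actor and unhides the Botte and Guding actors in its place.
; It then flags the cylinder as placed and notifies the UI actor for the current game mode: SecurityUIActor under FireGameMode, only the first time, or ZhylBottleUIactor under BP_ZongHeGameMode.
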(event OnComponentBeginOverlap(Box)
  (params (OverlappedComponent :type Primitive%20Component%20Object%20Reference) (OtherActor :type Actor%20Object%20Reference) (OtherComp :type Primitive%20Component%20Object%20Reference) (OtherBodyIndex :type Integer) (bFromSweep :type Boolean) (SweepResult :type Hit%20Result%20Structure%20%28by%20ref%29))
  (bind _securityuiactor (Variables|Default|GetSecurityUIActor))
  (bind _zhylbottleuiactor (Variables|Default|GetzhylBottleUIactor))
  (bind _asbp_fire_yi_que_ping (Utilities|Casting|CastToBP_FireYiQuePing OtherActor))
  (Actor|DestroyActor _asbp_fire_yi_que_ping)
  (Rendering|SetActorHiddenInGame (Variables|Default|Getbotte) false)
  (Rendering|SetActorHiddenInGame (Variables|Default|Getguding) false)
  (Utilities|Casting|CastToFireGameMode (Game|GetGameMode)
    (:then
      (if (not (Variables|/Game/BluePrint/FireWork/SecurityUIIActor.SecurityUIIActor_C|GetIsYiQuePING _securityuiactor))
        (Variables|/Game/BluePrint/FireWork/SecurityUIIActor.SecurityUIIActor_C|SetIsYiQuePING _securityuiactor true)
        (Default|BottleCorrect _securityuiactor)))
    (:CastFailed
      (Utilities|Casting|CastToBP_ZongHeGameMode (Game|GetGameMode))
      (Variables|/Game/BluePrint/ZongHeYanLian/zhylBottleUIActor1.zhylBottleUIActor1_C|SetzhylIsYiQuePing _zhylbottleuiactor true)
      (Default|BottleUIyichu _zhylbottleuiactor))))

(event EventBeginPlay)

(event Collision|EventActorBeginOverlap
  (params (OtherActor :type Actor%20Object%20Reference)))

(event EventTick
  (params (DeltaSeconds :type Float%20%28single-precision%29)))

(fn ConstructionScript)