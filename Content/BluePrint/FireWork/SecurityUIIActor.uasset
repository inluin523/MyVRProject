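; SecurityUIIActor is a UI actor that tracks two preparation checks in a fire simulation and reports them to FireGameMode.
; SecurityCompelte hides its widget and marks security correct once rope, medkit and fire extinguisher flags are all set.
; BottleCorrect, when both gas-bottle flags are set, marks bottles correct, hides BottleUIActor and calls ConfirmButton's CheckWorkBefore.
; Each event acts only while its game mode flag is still false.
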(event Custom|SecurityCompelte
  (bind _asfire_game_mode (Utilities|Casting|CastToFireGameMode (Game|GetGameMode)))
  (if (not (Variables|/Game/BluePrint/FireGameMode.FireGameMode_C|GetIsSecurityCorrect _asfire_game_mode))
    (if (Math|Boolean|ANDBoolean (Variables|Default|GetIsRoopCorrect) (Variables|Default|GetIsMedkitCorrect) (Variables|Default|GetIsFireExtinguisherCorrect))
      (Rendering|SetVisibility (Variables|Default|GetWidget) false false)
      (Variables|/Game/BluePrint/FireGameMode.FireGameMode_C|SetIsSecurityCorrect _asfire_game_mode true))))

(event Custom|BottleCorrect
  (if (and (Variables|Default|GetIsYangQiPING) (Variables|Default|GetIsYiQuePING))
    (bind _asfire_game_mode (Utilities|Casting|CastToFireGameMode (Game|GetGameMode)))
    (if (not (Variables|/Game/BluePrint/FireGameMode.FireGameMode_C|GetIsBottleCorrect _asfire_game_mode))
      (Variables|/Game/BluePrint/FireGameMode.FireGameMode_C|SetIsBottleCorrect _asfire_game_mode true)
      (Rendering|SetActorHiddenInGame (Variables|Default|GetBottleUIActor) true)
      (Default|CheckWorkBefore (Variables|Default|GetConfirmButton)))))

(event EventBeginPlay)

(event Collision|EventActorBeginOverlap
  (params (OtherActor :type Actor%20Object%20Reference)))

(event EventTick
  (params (DeltaSeconds :type Float%20%28single-precision%29)))

(fn ConstructionScript)