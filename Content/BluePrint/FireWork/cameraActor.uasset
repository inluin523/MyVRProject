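; A firework-level trigger actor that swaps camera actors and shows a timed hint when its Box is overlapped.
; The overlap only acts while the FireGameMode IsCamera flag is set, hiding the first camera actor and revealing the second.
; It also sets the game mode's in-work and camera-start flags, then hides the hint actor again after a one-minute delay.
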(event OnComponentBeginOverlap(Box)
  (params (OverlappedComponent :type Primitive%20Component%20Object%20Reference) (OtherActor :type Actor%20Object%20Reference) (OtherComp :type Primitive%20Component%20Object%20Reference) (OtherBodyIndex :type Integer) (bFromSweep :type Boolean) (SweepResult :type Hit%20Result%20Structure%20%28by%20ref%29))
  (bind _dhzytishiactor (Variables|Default|GetdhzytishiActor))
  (bind _asfire_game_mode (Utilities|Casting|CastToFireGameMode (Game|GetGameMode)))
  (if (Variables|/Game/BluePrint/FireGameMode.FireGameMode_C|GetIsCamera _asfire_game_mode)
    (Rendering|SetActorHiddenInGame (Variables|Default|Getdhzyecameraactor1) true)
    (Rendering|SetActorHiddenInGame (Variables|Default|Getdhzycameraactor2) false)
    (Variables|/Game/BluePrint/FireGameMode.FireGameMode_C|SetisInWork _asfire_game_mode true)
    (Rendering|SetActorHiddenInGame _dhzytishiactor false)
    (Variables|/Game/BluePrint/FireGameMode.FireGameMode_C|SetISSTARTCAREMER _asfire_game_mode true)
    (Utilities|FlowControl|Delay 6e+01)
    (Rendering|SetActorHiddenInGame _dhzytishiactor true)))

(fn ConstructionScript)