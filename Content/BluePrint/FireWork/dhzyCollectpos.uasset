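; Collection point for the fire-work scenario that checks equipment is brought back once the game mode's IsAfterWork is set.
; Box overlaps latch a flag for the fire extinguisher, med kit, rope, blind plate (MangBan) and blind plate sign, identified by casts.
; Each match runs CheckClear, which, when all five are set, swaps visibility of referenced prompt and screen actors and enables confirmation through ConfirmUIUI.IsCanQueRen.
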(event OnComponentBeginOverlap(Box)
  (params (OverlappedComponent :type Primitive%20Component%20Object%20Reference) (OtherActor :type Actor%20Object%20Reference) (OtherComp :type Primitive%20Component%20Object%20Reference) (OtherBodyIndex :type Integer) (bFromSweep :type Boolean) (SweepResult :type Hit%20Result%20Structure%20%28by%20ref%29))
  (bind _asfire_game_mode (Utilities|Casting|CastToFireGameMode (Game|GetGameMode)))
  (if (Variables|/Game/BluePrint/FireGameMode.FireGameMode_C|GetisAfterWork _asfire_game_mode)
    (Utilities|FlowControl|Sequence
      (:then_0
        (Utilities|Casting|CastToMedkit OtherActor)
        (Variables|Default|SetHasMedKit true)
        (CallFunction|CheckClear))
      (:then_1
        (Utilities|Casting|CastToRoop OtherActor)
        (Variables|Default|SetHasRoop true)
        (CallFunction|CheckClear))
      (:then_2
        (Utilities|Casting|CastToTestDHFireExtinguisher1 OtherActor)
        (Variables|Default|SetHasFireExting true)
        (CallFunction|CheckClear))
      (:then_3
        (Utilities|Casting|CastToMangBanBiaoZhiActorPos OtherActor)
        (Variables|Default|SetHasMangBanBS true)
        (CallFunction|CheckClear))
      (:then_4
        (Utilities|Casting|CastToMangBan OtherActor)
        (Variables|Default|SetHasMangBan true)
        (CallFunction|CheckClear)))))

(event Custom|CheckClear
  (Utilities|Casting|CastToFireGameMode (Game|GetGameMode))
  (if (Math|Boolean|ANDBoolean (Variables|Default|GetHasFireExting) (Variables|Default|GetHasMedKit) (Variables|Default|GetHasRoop) (Variables|Default|GetHasMangBan) (Variables|Default|GetHasMangBanBS))
    (Rendering|SetActorHiddenInGame (Variables|Default|Getsecsec) true)
    (Rendering|SetActorHiddenInGame (Variables|Default|GetconfirmBT4) false)
    (Variables|/Game/BluePrint/FireWork/BP_ConfirmButton.BP_ConfirmButton_C|SetisCanQueRen (Variables|Default|GetconfirmUIUI) true)
    (Rendering|SetActorHiddenInGame (Variables|Default|Gettvactor10) true)
    (Rendering|SetActorHiddenInGame (Variables|Default|Gettvuiactor8) false)))

(fn ConstructionScript)