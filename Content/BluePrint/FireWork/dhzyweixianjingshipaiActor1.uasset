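; Trigger actor for a warning-sign step, apparently in a hazardous hot-work safety scenario, that advances the scene on overlap.
; When a dhzyweixianBSBlueprint1 actor enters the Box, it hides that actor's Widget and unhides each cordon actor in the Jingjiexian1 array.
; The same loop body swaps Tvui1 for Tvui2 and shows ConfirmBt, so those changes repeat per element and are skipped if the array is empty.
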(event OnComponentBeginOverlap(Box)
  (params (OverlappedComponent :type Primitive%20Component%20Object%20Reference) (OtherActor :type Actor%20Object%20Reference) (OtherComp :type Primitive%20Component%20Object%20Reference) (OtherBodyIndex :type Integer) (bFromSweep :type Boolean) (SweepResult :type Hit%20Result%20Structure%20%28by%20ref%29))
  (bind _asdhzyweixian_bsblueprint_1 (Utilities|Casting|CastTodhzyweixianBSBlueprint1 OtherActor))
  (Rendering|SetVisibility (Variables|/Game/BluePrint/FireWork/dhzyweixianBSBlueprint1.dhzyweixianBSBlueprint1_C|GetWidget _asdhzyweixian_bsblueprint_1) false false)
  (for _array_element (Variables|Default|Getjingjiexian1)
    (Rendering|SetActorHiddenInGame _array_element false)
    (Rendering|SetActorHiddenInGame (Variables|Default|Gettvui1) true)
    (Rendering|SetActorHiddenInGame (Variables|Default|Gettvui2) false)
    (Rendering|SetActorHiddenInGame (Variables|Default|Getconfirm_bt) false)))

(event EventBeginPlay)

(event Collision|EventActorBeginOverlap
  (params (OtherActor :type Actor%20Object%20Reference)))

(event EventTick
  (params (DeltaSeconds :type Float%20%28single-precision%29)))

(fn ConstructionScript)