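; Camera prop actor in the FireWork folder, with Pickup and Drop events and an on-screen text cue.
; Any overlap with its Box switches the shexiangji widget on its widget component from the first text block to the second.
; Drop re-enables mesh physics and detaches the actor, keeping its world transform.
; Pickup does nothing: the logic to disable physics and attach to a given component is unconnected.
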(event OnComponentBeginOverlap(Box)
  (params (OverlappedComponent :type Primitive%20Component%20Object%20Reference) (OtherActor :type Actor%20Object%20Reference) (OtherComp :type Primitive%20Component%20Object%20Reference) (OtherBodyIndex :type Integer) (bFromSweep :type Boolean) (SweepResult :type Hit%20Result%20Structure%20%28by%20ref%29))
  (bind _asshexiangji (Utilities|Casting|CastToshexiangji (UserInterface|GetUserWidgetObject (Variables|Default|GetWidget))))
  (Widget|SetVisibility (Variables|/Game/UI/LimitSpace/UI/UMG/shexiangji.shexiangji_C|GetTextBlock_0 _asshexiangji) "Hidden")
  (Widget|SetVisibility (Variables|/Game/UI/LimitSpace/UI/UMG/shexiangji.shexiangji_C|GetTextBlock_1 _asshexiangji) "Visible"))

(event EventBeginPlay)

(event Collision|EventActorBeginOverlap
  (params (OtherActor :type Actor%20Object%20Reference)))

(event EventPickup
  (params (AttachTo :type Scene%20Component%20Object%20Reference) (CharacterType :type EcharacterType%20Enum :default "NewEnumerator0")))

(event EventTick
  (params (DeltaSeconds :type Float%20%28single-precision%29)))

(event EventDrop
  (Physics|SetSimulatePhysics (Variables|Default|GetStaticMesh) true)
  (Transformation|DetachFromActor "KeepWorld" "KeepWorld" "KeepWorld"))

(fn ConstructionScript)