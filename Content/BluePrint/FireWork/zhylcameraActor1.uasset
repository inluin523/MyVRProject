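; A trigger-box actor that switches the scene into a "Zhyl" work state when something overlaps it while the game mode's ZhylIsCamera flag is set.
; The overlap hides Zongheactor1 and reveals Zongheactor2 and ZhylStartWork.
; It also reveals the Han actor on the first qualifying overlap only, latched by ZhylisInWork.
; An actor spawn at Hanqiang's transform is left unconnected and never runs.
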(event OnComponentBeginOverlap(Box)
  (params (OverlappedComponent :type Primitive%20Component%20Object%20Reference) (OtherActor :type Actor%20Object%20Reference) (OtherComp :type Primitive%20Component%20Object%20Reference) (OtherBodyIndex :type Integer) (bFromSweep :type Boolean) (SweepResult :type Hit%20Result%20Structure%20%28by%20ref%29))
  (bind _asbp_zong_he_game_mode (Utilities|Casting|CastToBP_ZongHeGameMode (Game|GetGameMode)))
  (if (Variables|/Game/BluePrint/ZongHeYanLian/BP_ZongHeGameMode.BP_ZongHeGameMode_C|GetzhylIsCamera _asbp_zong_he_game_mode)
    (Rendering|SetActorHiddenInGame (Variables|Default|Getzongheactor1) true)
    (Rendering|SetActorHiddenInGame (Variables|Default|Getzongheactor2) false)
    (Rendering|SetActorHiddenInGame (Variables|Default|GetzhylStartWork) false)
    (if (not (Variables|Default|GetzhylisInWork))
      (Rendering|SetActorHiddenInGame (Variables|Default|Gethan) false)
      (Variables|Default|SetzhylisInWork true))))

(fn ConstructionScript)