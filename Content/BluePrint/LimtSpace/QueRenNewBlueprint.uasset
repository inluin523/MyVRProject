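; Confirm button for confined-space work training that steps through work declaration, permit issuing and final confirmation.
; Pickup picks the stage by boolean flags, slides the button along X with paired Timelines, then swaps prompt and TV actors, with Delays, from the second Timeline's Update.
; checkWorkBeforeQianFa unlocks issuing once five GameMode safety flags are true.
; Issuing sets GameMode after-work flags; final confirmation reveals Sxkjdengji and prints a score string.
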(event Custom|checkWorkBeforeQianFa
  (bind _aslimited_space_game_mode (Utilities|Casting|CastToLimitedSpaceGameMode (Game|GetGameMode)))
  (if (Math|Boolean|ANDBoolean (Variables|/Game/BluePrint/LimitedSpaceGameMode.LimitedSpaceGameMode_C|GetsxkjIsClearGarbge _aslimited_space_game_mode) (Variables|/Game/BluePrint/LimitedSpaceGameMode.LimitedSpaceGameMode_C|GetsxkjIsSecurityCorrect _aslimited_space_game_mode) (Variables|/Game/BluePrint/LimitedSpaceGameMode.LimitedSpaceGameMode_C|GetsxkjIsmangbanUI _aslimited_space_game_mode) (Variables|/Game/BluePrint/LimitedSpaceGameMode.LimitedSpaceGameMode_C|GetsxkjIsDetectGas _aslimited_space_game_mode) (Variables|/Game/BluePrint/LimitedSpaceGameMode.LimitedSpaceGameMode_C|GetsxkjIsAnQuanJuLi _aslimited_space_game_mode))
    (Variables|Default|SetisCanQianFa true)))

(event EventPickup
  (params (AttachTo :type Scene%20Component%20Object%20Reference) (CharacterType :type EcharacterType%20Enum :default "NewEnumerator0"))
  (bind _sxkjtvactor3 (Variables|Default|Getsxkjtvactor3))
  (bind _querenactor2 (Variables|Default|Getquerenactor2))
  (bind _querenactor9 (Variables|Default|Getquerenactor9))
  (bind _sxkjtvactor8 (Variables|Default|Getsxkjtvactor8))
  (bind _querenactor6 (Variables|Default|Getquerenactor6))
  (bind _querenactor10 (Variables|Default|Getquerenactor10))
  (bind _sxkjtvactor11 (Variables|Default|Getsxkjtvactor11))
  (bind _sxkjtvactor12 (Variables|Default|Getsxkjtvactor12))
  ;[1 1 1] 作业申报
  (if (Variables|Default|Getisbeforwork)
    (Variables|Default|Setisbeforwork false)
    (Rendering|SetActorHiddenInGame (Variables|Default|Getquerenactor1) true)
    (bind _新建轨迹_3 (Timeline|时间轴_0 Play)
      (:Update
        (Transformation|SetActorLocation (Math|Vector|MakeVector _新建轨迹_3 -9717.982422 98.60981) false false))
      (:Finished
        (bind _新建轨迹_3_2 (Timeline|时间轴_1 Play)
          (:Update
            (Transformation|SetActorLocation (Math|Vector|MakeVector _新建轨迹_3_2 -9717.982422 98.60981) false false)
            (Rendering|SetActorHiddenInGame (Variables|Default|Getsxkjtvactor2) true)
            (Rendering|SetActorHiddenInGame _sxkjtvactor3 false)
            (Rendering|SetActorHiddenInGame _querenactor2 false)
            (Utilities|FlowControl|Delay 5.0)
            (Rendering|SetActorHiddenInGame _querenactor2 true)
            (Rendering|SetActorHiddenInGame (Variables|Default|Getquerenactor3) false)
            (Rendering|SetActorHiddenInGame _sxkjtvactor3 true)
            (Rendering|SetActorHiddenInGame (Variables|Default|Getsxkjtvactor4) false)
            (Rendering|SetActorHiddenInGame (Variables|Default|GetsxkjFYactor) false)))))
    (elif (Variables|Default|GetisCanQianFa)
      (bind _新建轨迹_3_3 (Timeline|时间轴_2 Play)
        (:Update
          (Transformation|SetActorLocation (Math|Vector|MakeVector _新建轨迹_3_3 -9717.982422 98.60981) false false))
        (:Finished
          (bind _新建轨迹_3_4 (Timeline|时间轴_3 Play)
            (:Update
              (Transformation|SetActorLocation (Math|Vector|MakeVector _新建轨迹_3_4 -9717.982422 98.60981) false false)
              (Rendering|SetActorHiddenInGame (Variables|Default|Getsxkjtvactor7) true)
              (Rendering|SetActorHiddenInGame _sxkjtvactor8 false)
              (Variables|Default|SetisCanQianFa false)
              (Rendering|SetActorHiddenInGame (Variables|Default|Getquerenactor5) true)
              (Rendering|SetActorHiddenInGame _querenactor6 false)
              (Utilities|FlowControl|Delay 5.0)
              (Rendering|SetActorHiddenInGame _querenactor6 true)
              (Rendering|SetActorHiddenInGame (Variables|Default|Getquerenactor7) false)
              (Rendering|SetActorHiddenInGame _sxkjtvactor8 true)
              (Rendering|SetActorHiddenInGame (Variables|Default|Getsxkjtvactor9) false)
              (Rendering|SetActorHiddenInGame (Variables|Default|GetsxkjFYactor) false)
              (bind _aslimited_space_game_mode (Utilities|Casting|CastToLimitedSpaceGameMode (Game|GetGameMode)))
              (Variables|/Game/BluePrint/LimitedSpaceGameMode.LimitedSpaceGameMode_C|SetsxkjIsThirdFY _aslimited_space_game_mode true)
              (bind _aslimited_space_game_mode_2 (Utilities|Casting|CastToLimitedSpaceGameMode (Game|GetGameMode)))
              (Variables|/Game/BluePrint/LimitedSpaceGameMode.LimitedSpaceGameMode_C|SetsxkjIsCamera _aslimited_space_game_mode_2 true)
              (Variables|/Game/BluePrint/LimitedSpaceGameMode.LimitedSpaceGameMode_C|SetsxkjIsAfterWork _aslimited_space_game_mode_2 true)
              (Rendering|SetActorHiddenInGame (Variables|Default|Getsxkjcameraactor1) false)))))
      (elif (Variables|Default|GetsxkjIsCanQueRen)
        (bind _新建轨迹_3_5 (Timeline|时间轴_4 Play)
          (:Update
            (Transformation|SetActorLocation (Math|Vector|MakeVector _新建轨迹_3_5 -9717.982422 98.60981) false false))
          (:Finished
            (bind _新建轨迹_3_6 (Timeline|时间轴_5 Play)
              (:Update
                (Transformation|SetActorLocation (Math|Vector|MakeVector _新建轨迹_3_6 -9717.982422 98.60981) false false)
                (Variables|Default|SetsxkjIsCanQueRen false)
                (Rendering|SetActorHiddenInGame (Variables|Default|Getsxkjtvactor8) true)
                (Rendering|SetActorHiddenInGame (Variables|Default|Getquerenactor8) true)
                (Rendering|SetActorHiddenInGame _querenactor9 false)
                (Rendering|SetActorHiddenInGame _sxkjtvactor11 false)
                (Utilities|FlowControl|Delay 7.0)
                (Rendering|SetActorHiddenInGame _sxkjtvactor11 true)
                (Rendering|SetActorHiddenInGame _sxkjtvactor12 false)
                (Rendering|SetActorHiddenInGame _querenactor9 true)
                (Rendering|SetActorHiddenInGame _querenactor10 false)
                (Utilities|FlowControl|Delay 5.0)
                (Rendering|SetActorHiddenInGame _querenactor10 true)
                (Rendering|SetActorHiddenInGame _sxkjtvactor12 true)
                (Rendering|SetActorHiddenInGame (Variables|Default|Getsxkjdengji) false)
                (Development|PrintString "scorescore:100" false)))))))))

(fn ConstructionScript)