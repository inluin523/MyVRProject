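; Valve (famen) actor for a limited-space exercise, gating the valve UI step on its prerequisites.
; Until the GameMode's completion flag is set, famenUIyichu checks valve, sign, blind-plate and pipe-wrench flags.
; Success sets the flag, hides the widget, calls Sxkjfmss, then shows a hint actor temporarily after a delay.
; Otherwise it reveals what appear to be failure, score and valve-operation feedback actors.
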(event Custom|famenUIyichu
  (bind _sxkjtishiactor (Variables|Default|GetsxkjtishiActor))
  (bind _aslimited_space_game_mode (Utilities|Casting|CastToLimitedSpaceGameMode (Game|GetGameMode)))
  (if (not (Variables|/Game/BluePrint/LimitedSpaceGameMode.LimitedSpaceGameMode_C|GetsxkjIsmangbanUI _aslimited_space_game_mode))
    (if (Math|Boolean|ANDBoolean (Variables|Default|Getisfamen) (Variables|Default|Getisbiaoshi) (Variables|Default|Getismangban) (Variables|/Game/BluePrint/LimtSpace/guandaoActor.guandaoActor_C|Getisbanshou (Variables|Default|Getguandaobanshou)))
      (Variables|/Game/BluePrint/LimitedSpaceGameMode.LimitedSpaceGameMode_C|SetsxkjIsmangbanUI _aslimited_space_game_mode true)
      (Rendering|SetVisibility (Variables|Default|GetWidget) false false)
      (Default|Sxkjfmss (Variables|Default|Getsxkjfms))
      (Utilities|FlowControl|Delay 4.0)
      (Rendering|SetActorHiddenInGame _sxkjtishiactor false)
      (Utilities|FlowControl|Delay 6e+01)
      (Rendering|SetActorHiddenInGame _sxkjtishiactor true)
      (else
        (Rendering|SetActorHiddenInGame (Variables|Default|Getshaibaiactor) false)
        (Rendering|SetActorHiddenInGame (Variables|Default|Getsxkjscore) false)
        (Rendering|SetActorHiddenInGame (Variables|Default|Getfmczywactor) false)))))

(fn ConstructionScript)