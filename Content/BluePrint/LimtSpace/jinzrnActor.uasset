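; VR grabbable actor that a motion controller can pick up and drop, with position sync through the player controller.
; Pickup attaches it to the hand and starts a looping timer that sends an offset hand transform to MyPlayerController, flipping roll correction for a mirrored hand.
; Drop stops the timer, detaches and briefly simulates physics on the Cube.
; The Pos RepNotify applies non-zero replicated transforms to the Cube.
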(event Custom|UpdatePos_C
  (bind _self self)
  (bind _hand (Variables|Default|GetHand))
  (bind _cube (Variables|Default|GetCube))
  (bind _scene (Variables|Default|GetScene))
  (bind _returnvalue (Transformation|GetWorldTransform _hand))
  (bind _returnvalue_2 (Transformation|GetWorldLocation _cube))
  (bind _returnvalue_3 (Transformation|GetWorldLocation _scene))
  (bind _returnvalue_4 (- _returnvalue_2 _returnvalue_3))
  (bind (_roll _pitch _yaw) (Math|Rotator|BreakRotator (.rotation _returnvalue)))
  (bind _returnvalue_5 (+ (.location _returnvalue) _returnvalue_4))
  (bind _asmy_player_controller (Utilities|Casting|CastToMyPlayerController (Game|GetPlayerController 0)))
  (if (< (.Y (Math|Vector|BreakVector (.scale _returnvalue))) 0.0)
    (Default|UpdatePickUpPosC _asmy_player_controller _self (Math|Transform|MakeTransform _returnvalue_5 (Math|Rotator|MakeRotator (+ _roll 9e+01) _pitch _yaw) (Transformation|GetWorldScale (Variables|Default|GetScene))))
    (else
      (Default|UpdatePickUpPosC _asmy_player_controller _self (Math|Transform|MakeTransform _returnvalue_5 (Math|Rotator|MakeRotator (- _roll 9e+01) _pitch _yaw) (Transformation|GetWorldScale (Variables|Default|GetScene)))))))

(event Custom|SetPickUp_S
  (params (IsPickUp :type Boolean))
  ;[1 1 1] 设置物体被抓
  (Variables|Default|SetIsPickUp IsPickUp))

(event EventPickup
  (params (AttachTo :type Scene%20Component%20Object%20Reference) (CharacterType :type EcharacterType%20Enum :default "NewEnumerator0"))
  (Variables|Default|SetHand AttachTo)
  (Utilities|FlowControl|Sequence
    (:then_0
      (CallFunction|SetPickUpS false))
    (:then_1
      (Transformation|AttachComponentToComponent (VehicleSound|GetRootComponent) AttachTo "None" "KeepWorld" "KeepWorld" "KeepWorld" false))
    (:then_2
      ;[1 1 1] 心跳同步
      (Utilities|Time|SetTimerbyFunctionName 0 "UpdatePos" 0.05 true))))

(event EventDrop
  (bind _cube (Variables|Default|GetCube))
  (Utilities|FlowControl|Sequence
    (:then_0
      ;[1 1 1] 设置灭火器不被抓
      (CallFunction|SetPickUpS false))
    (:then_1
      ;[1 1 1] 取消心跳同步
      (Utilities|Time|ClearTimerbyFunctionName 0 "UpdatePos"))
    (:then_2
      (Transformation|DetachFromActor "KeepWorld" "KeepWorld" "KeepWorld")
      (Physics|SetSimulatePhysics _cube true)
      (Utilities|FlowControl|Delay 3.0)
      (Physics|SetSimulatePhysics _cube false))))

(fn ConstructionScript)

(fn OnRepPos
  (bind _pos (Variables|Default|Getpos))
  (if (Math|Vector|NotEqual(Vector) (.Location (Math|Transform|BreakTransform _pos)) "0, 0, 0" 0.1)
    (Transformation|SetWorldTransform (Variables|Default|GetCube) _pos false false)))

(fn UpdatePos
  (CallFunction|UpdatePosC))