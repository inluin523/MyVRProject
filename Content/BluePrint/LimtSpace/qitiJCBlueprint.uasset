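; Gas-detection checkpoint for a limited-space VR training scenario.
; When a motion controller with a visible detector enters the Sphere, it writes fixed readings to the detector screen and flags detection done in LimitedSpaceGameMode.
; It then checks three other game-mode flags, either advancing actors and starting the pre-work check or revealing failure and score actors.
; Separately, the Box swaps an overlapping jinzrnActor for a pre-placed hidden actor.
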(event OnComponentBeginOverlap(Sphere)
  (params (OverlappedComponent :type Primitive%20Component%20Object%20Reference) (OtherActor :type Actor%20Object%20Reference) (OtherComp :type Primitive%20Component%20Object%20Reference) (OtherBodyIndex :type Integer) (bFromSweep :type Boolean) (SweepResult :type Hit%20Result%20Structure%20%28by%20ref%29))
  (bind _asbp_motion_controller (Utilities|Casting|CastToBP_MotionController OtherActor))
  (bind _aslimited_space_game_mode (Utilities|Casting|CastToLimitedSpaceGameMode (Game|GetGameMode)))
  (if (not (Variables|/Game/BluePrint/LimitedSpaceGameMode.LimitedSpaceGameMode_C|GetsxkjIsDetectGas _aslimited_space_game_mode))
    (if (Rendering|IsVisible (Variables|/Game/BluePrint/BP_MotionController.BP_MotionController_C|GetGasDetection _asbp_motion_controller))
      (bind _asgas_detection_ui (Utilities|Casting|CastToGasDetectionUI (UserInterface|GetUserWidgetObject (Variables|/Game/BluePrint/BP_MotionController.BP_MotionController_C|GetScreen _asbp_motion_controller))))
      (Variables|/Game/UI/FireWork/GasDetectionUI.GasDetectionUI_C|SetExplodeLimitText _asgas_detection_ui "5%")
      (Variables|/Game/UI/FireWork/GasDetectionUI.GasDetectionUI_C|SetGasDetectionText _asgas_detection_ui "0.3%")
      (Variables|/Game/BluePrint/LimitedSpaceGameMode.LimitedSpaceGameMode_C|SetsxkjIsDetectGas _aslimited_space_game_mode true)
      (Default|Gasuiyichu (Variables|Default|GetGasDetectionUIyc))
      (CallFunction|Sxkjcheackwork))))

(event OnComponentBeginOverlap(Box)
  (params (OverlappedComponent :type Primitive%20Component%20Object%20Reference) (OtherActor :type Actor%20Object%20Reference) (OtherComp :type Primitive%20Component%20Object%20Reference) (OtherBodyIndex :type Integer) (bFromSweep :type Boolean) (SweepResult :type Hit%20Result%20Structure%20%28by%20ref%29))
  (Utilities|Casting|CastToLimitedSpaceGameMode (Game|GetGameMode))
  (bind _asjinzrn_actor (Utilities|Casting|CastTojinzrnActor OtherActor))
  (Actor|DestroyActor _asjinzrn_actor)
  (Rendering|SetActorHiddenInGame (Variables|Default|Getjinzhiactorpos) false))

(event Custom|sxkjcheackwork
  (bind _aslimited_space_game_mode (Utilities|Casting|CastToLimitedSpaceGameMode (Game|GetGameMode)))
  (if (Math|Boolean|ANDBoolean (Variables|/Game/BluePrint/LimitedSpaceGameMode.LimitedSpaceGameMode_C|GetsxkjIsClearGarbge _aslimited_space_game_mode) (Variables|/Game/BluePrint/LimitedSpaceGameMode.LimitedSpaceGameMode_C|GetsxkjIsSecurityCorrect _aslimited_space_game_mode) (Variables|/Game/BluePrint/LimitedSpaceGameMode.LimitedSpaceGameMode_C|GetsxkjIsmangbanUI _aslimited_space_game_mode))
    (Rendering|SetActorHiddenInGame (Variables|Default|Getquerenactor4) true)
    (Rendering|SetActorHiddenInGame (Variables|Default|Getquerenactor5) false)
    (Rendering|SetActorHiddenInGame (Variables|Default|Getsxkjtvactor5) true)
    (Rendering|SetActorHiddenInGame (Variables|Default|Getsxkjtvactor6) false)
    (Rendering|SetActorHiddenInGame (Variables|Default|Getsxkjfy) false)
    (bind _aslimited_space_game_mode_2 (Utilities|Casting|CastToLimitedSpaceGameMode (Game|GetGameMode)))
    (Variables|/Game/BluePrint/LimitedSpaceGameMode.LimitedSpaceGameMode_C|SetsxkjIsSecondFY _aslimited_space_game_mode_2 true)
    (Default|CheckWorkBeforeQianFa (Variables|Default|Getcheackworkbefore))
    (else
      (Rendering|SetActorHiddenInGame (Variables|Default|Getshibaiactor2222) false)
      (Rendering|SetActorHiddenInGame (Variables|Default|Getsxkjscore) false)
      (Rendering|SetActorHiddenInGame (Variables|Default|GetzyqcaywACTOR) false))))

(event EventBeginPlay)

(event Collision|EventActorBeginOverlap
  (params (OtherActor :type Actor%20Object%20Reference)))

(event EventTick
  (params (DeltaSeconds :type Float%20%28single-precision%29)))

(fn ConstructionScript)