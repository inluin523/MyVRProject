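; Collection-zone actor for a confined-space exercise that checks whether all required safety equipment has been brought to it.
; While the game mode's after-work and correct flags are set, box overlaps cast the incoming actor to six item types: extinguisher, medkit, rope, blind plate, blind-plate sign, searchlight.
; Each match latches a flag and runs CheckClear.
; Once all are set, CheckClear swaps prompt and TV actor visibility and enables confirmation in the UI.
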(event OnComponentBeginOverlap(Box)
  (params (OverlappedComponent :type Primitive%20Component%20Object%20Reference) (OtherActor :type Actor%20Object%20Reference) (OtherComp :type Primitive%20Component%20Object%20Reference) (OtherBodyIndex :type Integer) (bFromSweep :type Boolean) (SweepResult :type Hit%20Result%20Structure%20%28by%20ref%29))
  (bind _aslimited_space_game_mode (Utilities|Casting|CastToLimitedSpaceGameMode (Game|GetGameMode)))
  (if (and (Variables|/Game/BluePrint/LimitedSpaceGameMode.LimitedSpaceGameMode_C|GetsxkjIsAfterWork _aslimited_space_game_mode) (Variables|/Game/BluePrint/LimitedSpaceGameMode.LimitedSpaceGameMode_C|Getsxkjiscorrect _aslimited_space_game_mode))
    (Utilities|FlowControl|Sequence
      (:then_0
        (Utilities|Casting|CastToMedkit OtherActor)
        (Variables|Default|SetHasMedKit true)
        (CallFunction|CheckClear))
      (:then_1
        (Utilities|Casting|CastToRoop OtherActor)
        (Variables|Default|SetHasRoop true)
        (CallFunction|CheckClear))
      (:then_2
        (Utilities|Casting|CastToTestDHFireExtinguisher1 OtherActor)
        (Variables|Default|SetHasFireExting true)
        (CallFunction|CheckClear))
      (:then_3
        (Utilities|Casting|CastTosxkjMangBanBiaoZhiActorPos1 OtherActor)
        (Variables|Default|SetHasMangBanBS true)
        (CallFunction|CheckClear))
      (:then_4
        (Utilities|Casting|CastTosxkjMangBan1 OtherActor)
        (Variables|Default|SetHasMangBan true)
        (CallFunction|CheckClear))
      (:then_5
        (Utilities|Casting|CastTotanzhaodeng OtherActor)
        (Variables|Default|SetHasTanzhao true)
        (CallFunction|CheckClear)))))

(event Custom|CheckClear
  (if (Math|Boolean|ANDBoolean (Variables|Default|GetHasFireExting) (Variables|Default|GetHasMedKit) (Variables|Default|GetHasRoop) (Variables|Default|GetHasMangBan) (Variables|Default|GetHasMangBanBS) (Variables|Default|GetHasTanzhao))
    (Rendering|SetActorHiddenInGame (Variables|Default|Getsxkjaqqcactor1) true)
    (Rendering|SetActorHiddenInGame (Variables|Default|Getsxkjquerenactor8) false)
    (Variables|/Game/BluePrint/LimtSpace/QueRenNewBlueprint.QueRenNewBlueprint_C|SetsxkjIsCanQueRen (Variables|Default|GetconfirmUIUI) true)
    (Rendering|SetActorHiddenInGame (Variables|Default|Getsxkjtvactor10) true)
    (Rendering|SetActorHiddenInGame (Variables|Default|Getsxkjtvactor8) false)))

(fn ConstructionScript)