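; Page-turn actor for the LimitedSpace scenario that, on Pickup, animates itself and advances paired display actors through up to three stages.
; A local first-pick flag, then second and third page-turn flags on LimitedSpaceGameMode, select two chained timelines that slide it along X.
; Each second timeline's Update clears the flag and toggles TV and confirm actor visibility.
; The second stage also calls CheckWorkBeforeQianFa on the confirm UI every update.
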(event EventPickup
  (params (AttachTo :type Scene%20Component%20Object%20Reference) (CharacterType :type EcharacterType%20Enum :default "NewEnumerator0"))
  (if (Variables|Default|GetsxkjFirstPick)
    (bind _新建轨迹_3 (Timeline|时间轴_0 Play)
      (:Update
        (Transformation|SetActorLocation (Math|Vector|MakeVector _新建轨迹_3 -10135.648438 79.427124) false false))
      (:Finished
        (bind _新建轨迹_3_2 (Timeline|时间轴_1 Play)
          (:Update
            (Transformation|SetActorLocation (Math|Vector|MakeVector _新建轨迹_3_2 -10135.648438 79.427124) false false)
            (Variables|Default|SetsxkjFirstPick false)
            (Rendering|SetActorHiddenInGame (Variables|Default|Getsxkjtvactor4) true)
            (Rendering|SetActorHiddenInGame (Variables|Default|Getsxkjtvactor5) false)
            (Rendering|SetActorHiddenInGame (Variables|Default|Getquerenactor3) true)
            (Rendering|SetActorHiddenInGame (Variables|Default|Getquerenactor4) false)))))
    (else
      (bind _aslimited_space_game_mode (Utilities|Casting|CastToLimitedSpaceGameMode (Game|GetGameMode)))
      (if (Variables|/Game/BluePrint/LimitedSpaceGameMode.LimitedSpaceGameMode_C|GetsxkjIsSecondFY _aslimited_space_game_mode)
        (bind _新建轨迹_3_3 (Timeline|时间轴_2 Play)
          (:Update
            (Transformation|SetActorLocation (Math|Vector|MakeVector _新建轨迹_3_3 -10135.648438 79.427124) false false))
          (:Finished
            (bind _新建轨迹_3_4 (Timeline|时间轴_3 Play)
              (:Update
                (Transformation|SetActorLocation (Math|Vector|MakeVector _新建轨迹_3_4 -10135.648438 79.427124) false false)
                (Variables|/Game/BluePrint/LimitedSpaceGameMode.LimitedSpaceGameMode_C|SetsxkjIsSecondFY _aslimited_space_game_mode false)
                (Rendering|SetActorHiddenInGame (Variables|Default|Getsxkjtvactor6) true)
                (Rendering|SetActorHiddenInGame (Variables|Default|Getsxkjtvactor7) false)
                (Default|CheckWorkBeforeQianFa (Variables|Default|GetsxkjquerenUI))))))
        (elif (Variables|/Game/BluePrint/LimitedSpaceGameMode.LimitedSpaceGameMode_C|GetsxkjIsThirdFY _aslimited_space_game_mode)
          (bind _新建轨迹_3_5 (Timeline|时间轴_4 Play)
            (:Update
              (Transformation|SetActorLocation (Math|Vector|MakeVector _新建轨迹_3_5 -10135.648438 79.427124) false false))
            (:Finished
              (bind _新建轨迹_3_6 (Timeline|时间轴_5 Play)
                (:Update
                  (Transformation|SetActorLocation (Math|Vector|MakeVector _新建轨迹_3_6 -10135.648438 79.427124) false false)
                  (Variables|/Game/BluePrint/LimitedSpaceGameMode.LimitedSpaceGameMode_C|SetsxkjIsThirdFY _aslimited_space_game_mode false)
                  (Rendering|SetActorHiddenInGame (Variables|Default|Getsxkjtvactor9) true)
                  (Rendering|SetActorHiddenInGame (Variables|Default|Getsxkjtvactor10) false)
                  (Rendering|SetActorHiddenInGame (Variables|Default|Getquerenactor7) true))))))))))

(fn ConstructionScript)