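; Actor for the LimitedSpace scenario that shows a safety equipment sign widget and removes it once the equipment checks pass.
; Its custom event aqcqyc requires the rope, TangZD, medical and fire flags all to be true.
; It then sets SxkjIsSecurityCorrect on LimitedSpaceGameMode and hides the widget, skipping the work if that flag is already set.
; Nothing in this Blueprint calls the event.
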(event Custom|aqcqyc
  (bind _aslimited_space_game_mode (Utilities|Casting|CastToLimitedSpaceGameMode (Game|GetGameMode)))
  (if (not (Variables|/Game/BluePrint/LimitedSpaceGameMode.LimitedSpaceGameMode_C|GetsxkjIsSecurityCorrect _aslimited_space_game_mode))
    (if (Math|Boolean|ANDBoolean (Variables|Default|GetsxkjIsRoopCorrect) (Variables|Default|GetsxkjIsTangZDCorrect) (Variables|Default|GetsxkjIsMedicalCorrect) (Variables|Default|Getsxkjfire))
      (Variables|/Game/BluePrint/LimitedSpaceGameMode.LimitedSpaceGameMode_C|SetsxkjIsSecurityCorrect _aslimited_space_game_mode true)
      (Rendering|SetVisibility (Variables|Default|GetWidget) false false))))

(event EventBeginPlay)

(event Collision|EventActorBeginOverlap
  (params (OtherActor :type Actor%20Object%20Reference)))

(fn ConstructionScript)