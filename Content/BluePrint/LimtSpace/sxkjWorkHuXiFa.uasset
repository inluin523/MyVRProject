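; Trigger actor for a breathing-valve work step in a limited-space safety training level, checking which wrench overlaps its box.
; If the game mode's work state is active, the explosion-proof wrench runs a delayed sequence of showing and hiding staged actors, calls Mbss, flags the step correct and disarms.
; The ordinary wrench, or any overlap outside that state, reveals failure actors and logs a score string of 59.
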(event OnComponentBeginOverlap(Box)
  (params (OverlappedComponent :type Primitive%20Component%20Object%20Reference) (OtherActor :type Actor%20Object%20Reference) (OtherComp :type Primitive%20Component%20Object%20Reference) (OtherBodyIndex :type Integer) (bFromSweep :type Boolean) (SweepResult :type Hit%20Result%20Structure%20%28by%20ref%29))
  (bind _sxkjstartworkactor1 (Variables|Default|GetsxkjstartworkActor1))
  (bind _sxkjstartworkactor2 (Variables|Default|GetsxkjstartworkActor2))
  (if (Variables|Default|Getisfirst)
    (bind _aslimited_space_game_mode (Utilities|Casting|CastToLimitedSpaceGameMode (Game|GetGameMode)))
    (if (Variables|/Game/BluePrint/LimitedSpaceGameMode.LimitedSpaceGameMode_C|GetsxkjIsInwORK _aslimited_space_game_mode)
      (Utilities|Casting|CastTobanShouActorFanBao OtherActor
        (:then
          (Utilities|FlowControl|Delay 5.0)
          (Rendering|SetActorHiddenInGame (Variables|Default|Getsxkjworkactor3) true)
          (Rendering|SetActorHiddenInGame (Variables|Default|Getsxkjworkactor1) false)
          (Rendering|SetActorHiddenInGame (Variables|Default|GetsxkjWorkUI) true)
          (Rendering|SetActorHiddenInGame _sxkjstartworkactor1 false)
          (Utilities|FlowControl|Delay 15.0)
          (Rendering|SetActorHiddenInGame _sxkjstartworkactor1 true)
          (Rendering|SetActorHiddenInGame _sxkjstartworkactor2 false)
          (Utilities|FlowControl|Delay 1e+01)
          (Rendering|SetActorHiddenInGame _sxkjstartworkactor2 true)
          (Rendering|SetActorHiddenInGame (Variables|Default|GetsxkjaqqcActor1) false)
          (Default|Sxkjfmsyk (Variables|Default|Getmbss))
          (Variables|/Game/BluePrint/LimitedSpaceGameMode.LimitedSpaceGameMode_C|Setsxkjiscorrect _aslimited_space_game_mode true)
          (Variables|Default|Setisfirst false))
        (:CastFailed
          (Utilities|Casting|CastTobanShouActor OtherActor)
          (Rendering|SetActorHiddenInGame (Variables|Default|Getsxkjworkactor3) true)
          (Rendering|SetActorHiddenInGame (Variables|Default|Getsxkjworkactor2) false)
          (Rendering|SetActorHiddenInGame (Variables|Default|Getfanbaoactor) true)
          (Rendering|SetActorHiddenInGame (Variables|Default|Getshibaiactor3333) false)
          (Rendering|SetActorHiddenInGame (Variables|Default|Getbanshoutie) true)
          (Development|PrintString "scorescore:59" false)))
      (else
        (Rendering|SetActorHiddenInGame (Variables|Default|Getshibaiactor2222) false)
        (Rendering|SetActorHiddenInGame (Variables|Default|Getfanbaoactor) true)
        (Rendering|SetActorHiddenInGame (Variables|Default|Getbanshoutie) true)
        (Development|PrintString "scorescore:59" false)))))

(event EventBeginPlay)

(event Collision|EventActorBeginOverlap
  (params (OtherActor :type Actor%20Object%20Reference)))

(event EventTick
  (params (DeltaSeconds :type Float%20%28single-precision%29)))

(fn ConstructionScript)