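; Trigger actor for the limited-space scenario that reacts when a VR motion controller enters its box.
; If the LimitedSpaceGameMode camera flag is set, it hides the first camera actor and shows the second one plus the start-work UI.
; It then marks the game mode's in-work state as true.
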(event OnComponentBeginOverlap(Box)
  (params (OverlappedComponent :type Primitive%20Component%20Object%20Reference) (OtherActor :type Actor%20Object%20Reference) (OtherComp :type Primitive%20Component%20Object%20Reference) (OtherBodyIndex :type Integer) (bFromSweep :type Boolean) (SweepResult :type Hit%20Result%20Structure%20%28by%20ref%29))
  (Utilities|Casting|CastToBP_MotionController OtherActor)
  (bind _aslimited_space_game_mode (Utilities|Casting|CastToLimitedSpaceGameMode (Game|GetGameMode)))
  (if (Variables|/Game/BluePrint/LimitedSpaceGameMode.LimitedSpaceGameMode_C|GetsxkjIsCamera _aslimited_space_game_mode)
    (Rendering|SetActorHiddenInGame (Variables|Default|Getsxkjcameraactor1) true)
    (Rendering|SetActorHiddenInGame (Variables|Default|Getsxkjcameraactor2) false)
    (Rendering|SetActorHiddenInGame (Variables|Default|GetStartWorkUI) false)
    (Variables|/Game/BluePrint/LimitedSpaceGameMode.LimitedSpaceGameMode_C|SetsxkjIsInwORK _aslimited_space_game_mode true)))

(fn ConstructionScript)