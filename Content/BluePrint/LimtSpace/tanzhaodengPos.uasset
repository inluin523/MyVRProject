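; Target-position trigger for the searchlight (tanzhaodeng) in the limited-space scenario, marking it as correctly placed.
; When a tanzhaodeng actor overlaps the Box, it sets the searchlight flag on a security UI actor and calls Aqcqyc, skipping both if already set.
; The active game mode selects the UI actor and flag: LimitedSpaceGameMode uses SecurityUIActor, BP_ZongHeGameMode uses SeutyUIyichu.
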(event OnComponentBeginOverlap(Box)
  (params (OverlappedComponent :type Primitive%20Component%20Object%20Reference) (OtherActor :type Actor%20Object%20Reference) (OtherComp :type Primitive%20Component%20Object%20Reference) (OtherBodyIndex :type Integer) (bFromSweep :type Boolean) (SweepResult :type Hit%20Result%20Structure%20%28by%20ref%29))
  (bind _securityuiactor (Variables|Default|GetSecurityUIActor))
  (bind _seutyuiyichu (Variables|Default|GetseutyUIyichu))
  (Utilities|Casting|CastToLimitedSpaceGameMode (Game|GetGameMode)
    (:then
      (Utilities|Casting|CastTotanzhaodeng OtherActor)
      (if (not (Variables|/Game/BluePrint/LimtSpace/sxkjSecurityUIIActor1.sxkjSecurityUIIActor1_C|GetsxkjIsTangZDCorrect _securityuiactor))
        (Variables|/Game/BluePrint/LimtSpace/sxkjSecurityUIIActor1.sxkjSecurityUIIActor1_C|SetsxkjIsTangZDCorrect _securityuiactor true)
        (Default|Aqcqyc _securityuiactor)))
    (:CastFailed
      (Utilities|Casting|CastToBP_ZongHeGameMode (Game|GetGameMode))
      (Utilities|Casting|CastTotanzhaodeng OtherActor)
      (if (not (Variables|/Game/BluePrint/ZongHeYanLian/zhylSecurityUIIActor2.zhylSecurityUIIActor2_C|GetzhylisTanzhaodeng _seutyuiyichu))
        (Variables|/Game/BluePrint/ZongHeYanLian/zhylSecurityUIIActor2.zhylSecurityUIIActor2_C|SetzhylisTanzhaodeng _seutyuiyichu true)
        (Default|Aqcqyc _seutyuiyichu)))))

(event EventBeginPlay)

(fn ConstructionScript)