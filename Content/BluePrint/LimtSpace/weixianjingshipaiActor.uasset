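; Danger warning sign actor for a confined-space safety scenario that reacts when a weixianBSBlueprint actor enters its box.
; The overlap hides that actor's widget, then checks the safe-distance flag on LimitedSpaceGameMode.
; If the flag is unset, it swaps the two TV actors and reveals the cordon actors.
; The flag and confirm button reveal are set inside that loop, so both depend on a non-empty cordon array.
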(event OnComponentBeginOverlap(Box)
  (params (OverlappedComponent :type Primitive%20Component%20Object%20Reference) (OtherActor :type Actor%20Object%20Reference) (OtherComp :type Primitive%20Component%20Object%20Reference) (OtherBodyIndex :type Integer) (bFromSweep :type Boolean) (SweepResult :type Hit%20Result%20Structure%20%28by%20ref%29))
  (bind _asweixian_bsblueprint (Utilities|Casting|CastToweixianBSBlueprint OtherActor))
  (Rendering|SetVisibility (Variables|/Game/BluePrint/LimtSpace/weixianBSBlueprint.weixianBSBlueprint_C|GetWidget _asweixian_bsblueprint) false false)
  (bind _aslimited_space_game_mode (Utilities|Casting|CastToLimitedSpaceGameMode (Game|GetGameMode)))
  (if (not (Variables|/Game/BluePrint/LimitedSpaceGameMode.LimitedSpaceGameMode_C|GetsxkjIsAnQuanJuLi _aslimited_space_game_mode))
    (Rendering|SetActorHiddenInGame (Variables|Default|Getsxkjtvactor1) true)
    (Rendering|SetActorHiddenInGame (Variables|Default|Getsxkjtvactor2) false)
    (for _array_element (Variables|Default|GetJingjieActor)
      (Rendering|SetActorHiddenInGame _array_element false)
      (Variables|/Game/BluePrint/LimitedSpaceGameMode.LimitedSpaceGameMode_C|SetsxkjIsAnQuanJuLi _aslimited_space_game_mode true)
      (Rendering|SetActorHiddenInGame (Variables|Default|GetquerenBT) false))))

(event EventBeginPlay)

(event Collision|EventActorBeginOverlap
  (params (OtherActor :type Actor%20Object%20Reference)))

(event EventTick
  (params (DeltaSeconds :type Float%20%28single-precision%29)))

(fn ConstructionScript)

(fn OnRepTvUI)