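; Game instance Blueprint that hosts and joins LAN multiplayer sessions for work scenarios such as confined space and hot work.
; Three host events each create an eight-connection session and open a listen-server level from the immediate exec output, not a success callback.
; ZongHe and LimitGame both load LimitSpace, while HostGame takes a level name.
; JoinGame joins the given session only when Level is Firework, and results print on screen.
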(event Custom|HostGame
  (params (levelName :type Name))
  (|Session (Game|GetPlayerController 0) 8 true
    (:then
      (Game|OpenLevel(byName) levelName true "listen")
      (Development|PrintString "创建服务器成功" true true "(R=0.000000,G=0.660000,B=1.000000,A=1.000000)" 1e+01))
    (:OnFailure
      (Development|PrintString "创建服务器失败" true true "(R=0.000000,G=0.660000,B=1.000000,A=1.000000)" 1e+01))))

(event Custom|ZongHe
  (|Session (Game|GetPlayerController 0) 8 true
    (:then
      (Game|OpenLevel(byName) "LimitSpace" true "listen")
      (Development|PrintString "创建服务器成功" true true "(R=0.000000,G=0.660000,B=1.000000,A=1.000000)" 1e+01))
    (:OnFailure
      (Development|PrintString "创建服务器失败" true true "(R=0.000000,G=0.660000,B=1.000000,A=1.000000)" 1e+01))))

(event Custom|JoinGame
  (params (Session :type Blueprint%20Session%20Result%20Structure))
  (switch Utilities|FlowControl|Switch|SwitchonlevelSelectEnum (Variables|Default|Getlevel)
    (:NewEnumerator0
      (|JoinSession (Game|GetPlayerController 0) Session
        (:OnSuccess
          (Development|PrintString "加入服务器成功" true true "(R=0.000000,G=0.660000,B=1.000000,A=1.000000)" 1e+01))
        (:OnFailure
          (Development|PrintString "加入服务器失败" true true "(R=0.000000,G=0.660000,B=1.000000,A=1.000000)" 1e+01))))))

(event Custom|LimitGame
  (|Session (Game|GetPlayerController 0) 8 true
    (:then
      (Game|OpenLevel(byName) "LimitSpace" true "listen")
      (Development|PrintString "创建服务器成功" true true "(R=0.000000,G=0.660000,B=1.000000,A=1.000000)" 1e+01))
    (:OnFailure
      (Development|PrintString "创建服务器失败" true true "(R=0.000000,G=0.660000,B=1.000000,A=1.000000)" 1e+01))))