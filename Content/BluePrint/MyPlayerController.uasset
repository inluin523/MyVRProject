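; VR player controller that forwards grab, teleport and controller-switch input to the possessed MotionControllerPawn and drives its headset and hand position sync each Tick.
; Post-login events ask the ZongHe, Fire or LimitedSpace game mode to respawn the player.
; Held-prop transforms pass through a client/server-named event pair, where a cast sequence writes non-zero positions to each supported prop class.
; The TeleportFun function is an empty stub with unreachable leftover logic.
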(event Custom|ClientPostLogin
  (bind _asfire_game_mode (Utilities|Casting|CastToFireGameMode (Game|GetGameMode)))
  (Default|RespawnPlayerEvent _asfire_game_mode self))

(event Custom|sxkjclient
  (bind _aslimited_space_game_mode (Utilities|Casting|CastToLimitedSpaceGameMode (Game|GetGameMode)))
  (Default|RespawnPlayerEvent _aslimited_space_game_mode self))

(event Custom|ZHZYPostLogin
  ;[1 1 1] 注释
  (bind _asbp_zong_he_game_mode (Utilities|Casting|CastToBP_ZongHeGameMode (Game|GetGameMode)))
  (Default|RespawnPlayerEvent _asbp_zong_he_game_mode self))

(event Custom|DoSwitchController
  (bind (_ishave _character) (CallFunction|GetVRCharacter))
  (if _ishave
    (Default|DoSwitchController _character)))

(event Custom|GrabFun
  (params (IsLeft :type Boolean) (IsPressed_ :type Boolean))
  (bind (_ishave _character) (CallFunction|GetVRCharacter))
  (if _ishave
    (if IsLeft
      (Default|LeftGrabFun _character IsPressed_)
      (else
        (Default|RightGrabFun _character IsPressed_)))))

(event Input|ActionEvents|InputActionGrabLeft
  (params (Key :type Key%20Structure))
  (:Pressed
    (CallFunction|GrabFun true true))
  (:Released
    (CallFunction|GrabFun true false)))

(event Input|ActionEvents|InputActionGrabRight
  (params (Key :type Key%20Structure))
  (:Pressed
    (CallFunction|GrabFun false true))
  (:Released
    (CallFunction|GrabFun false false)))

(event Input|ActionEvents|InputActionSwitchController
  (params (Key :type Key%20Structure))
  (:Pressed
    (CallFunction|DoSwitchController)))

(event Custom|SynPos
  ;[1 1 1] 注释
  (bind (_ishave _character) (CallFunction|GetVRCharacter))
  (if _ishave
    (Default|SynPosC _character)))

(event EventTick
  (params (DeltaSeconds :type Float%20%28single-precision%29))
  (CallFunction|SynPos))

(event Custom|TeleporFun
  (params (IsLeft :type Boolean) (IsPressed_ :type Boolean))
  ;[1 1 1] 瞬移操作
  ;;[1 1 1] 注释
  (bind (_ishave _character) (CallFunction|GetVRCharacter))
  (if _ishave
    (if IsLeft
      (Default|LeftTeleportFun _character IsPressed_)
      (else
        (Default|RightTeleportFun _character IsPressed_)))))

(event Input|ActionEvents|InputActionTeleportRight
  (params (Key :type Key%20Structure))
  ;[1 1 1] 瞬移操作
  ;;[1 1 1] 右手瞬移
  (:Pressed
    (CallFunction|TeleporFun false true))
  (:Released
    (CallFunction|TeleporFun false false)))

(event Input|ActionEvents|InputActionTeleportLeft
  (params (Key :type Key%20Structure))
  ;[1 1 1] 瞬移操作
  ;;[1 1 1] 左手瞬移
  (:Pressed
    (CallFunction|TeleporFun true true))
  (:Released
    (CallFunction|TeleporFun true false)))

(event Custom|UpdatePickUpPos_S
  (params (actor :type Actor%20Object%20Reference) (pos :type Transform) (testpos :type Transform) (roppos :type Transform) (jinshipai :type Transform) (dhGarbage :type Transform) (mangban :type Transform) (banshoutie :type Transform) (sxkjmangban :type Transform) (sxkjweilan :type Transform) (sxkjtanzhaodeng :type Transform) (sxkjinzhi :type Transform) (sxkjfanbaobs :type Transform) (zhylweilan :type Transform) (zongheMediket :type Transform) (zonghemangban :type Transform) (yangqiping :type Transform) (yiyueping :type Transform) (Hanqiang :type Transform) (zongheMieHuo :type Transform))
  (Utilities|FlowControl|Sequence
    (:then_0
      (bind _astest_dhfire_extinguisher_1 (Utilities|Casting|CastToTestDHFireExtinguisher1 actor))
      (if (Math|Vector|NotEqual(Vector) (.Location (Math|Transform|BreakTransform pos)) "0, 0, 0" 0.0001)
        (Variables|/Game/BluePrint/FireWork/TestDHFireExtinguisher1.TestDHFireExtinguisher1_C|SetPos _astest_dhfire_extinguisher_1 pos)))
    (:then_1
      (bind _asmedkit (Utilities|Casting|CastToMedkit actor))
      (if (Math|Vector|NotEqual(Vector) (.Location (Math|Transform|BreakTransform testpos)) "0, 0, 0" 0.0001)
        (Variables|/Game/BluePrint/FireWork/Medkit.Medkit_C|Setpos _asmedkit testpos)))
    (:then_2
      (bind _asroop (Utilities|Casting|CastToRoop actor))
      (if (Math|Vector|NotEqual(Vector) (.Location (Math|Transform|BreakTransform roppos)) "0, 0, 0" 0.0001)
        (Variables|/Game/BluePrint/FireWork/Roop.Roop_C|SetroopPOS _asroop roppos)))
    (:then_3
      (bind _asdhzyweixian_bsblueprint_1 (Utilities|Casting|CastTodhzyweixianBSBlueprint1 actor))
      (if (Math|Vector|NotEqual(Vector) (.Location (Math|Transform|BreakTransform jinshipai)) "0, 0, 0" 0.0001)
        (Variables|/Game/BluePrint/FireWork/dhzyweixianBSBlueprint1.dhzyweixianBSBlueprint1_C|Setpos _asdhzyweixian_bsblueprint_1 jinshipai)))
    (:then_4
      (bind _asbp_garbage (Utilities|Casting|CastToBP_Garbage actor))
      (if (Math|Vector|NotEqual(Vector) (.Location (Math|Transform|BreakTransform dhGarbage)) "0, 0, 0" 0.0001)
        (Variables|/Game/ceTest/BP_Garbage.BP_Garbage_C|Setpos _asbp_garbage dhGarbage)))
    (:then_5
      (bind _asmang_ban (Utilities|Casting|CastToMangBan actor))
      (if (Math|Vector|NotEqual(Vector) (.Location (Math|Transform|BreakTransform mangban)) "0, 0, 0" 0.0001)
        (Variables|/Game/BluePrint/FireWork/MangBan.MangBan_C|Setpos _asmang_ban mangban)))
    (:then_6
      (bind _asban_shou_actor (Utilities|Casting|CastTobanShouActor actor))
      (if (Math|Vector|NotEqual(Vector) (.Location (Math|Transform|BreakTransform banshoutie)) "0, 0, 0" 0.0001)
        (Variables|/Game/BluePrint/FireWork/banShouActor.banShouActor_C|Setpos _asban_shou_actor banshoutie)))
    (:then_7
      (bind _assxkj_mang_ban_1 (Utilities|Casting|CastTosxkjMangBan1 actor))
      (if (Math|Vector|NotEqual(Vector) (.Location (Math|Transform|BreakTransform sxkjmangban)) "0, 0, 0" 0.0001)
        (Variables|/Game/BluePrint/LimtSpace/sxkjMangBan1.sxkjMangBan1_C|Setpos _assxkj_mang_ban_1 sxkjmangban)))
    (:then_8
      (bind _asweixian_bsblueprint (Utilities|Casting|CastToweixianBSBlueprint actor))
      (if (Math|Vector|NotEqual(Vector) (.Location (Math|Transform|BreakTransform sxkjweilan)) "0, 0, 0" 0.0001)
        (Variables|/Game/BluePrint/LimtSpace/weixianBSBlueprint.weixianBSBlueprint_C|Setpos _asweixian_bsblueprint sxkjweilan)))
    (:then_9
      (bind _astanzhaodeng (Utilities|Casting|CastTotanzhaodeng actor))
      (if (Math|Vector|NotEqual(Vector) (.Location (Math|Transform|BreakTransform sxkjtanzhaodeng)) "0, 0, 0" 0.0001)
        (Variables|/Game/BluePrint/FireWork/tanzhaodeng.tanzhaodeng_C|Setpos _astanzhaodeng sxkjtanzhaodeng)))
    (:then_10
      (bind _asjinzrn_actor (Utilities|Casting|CastTojinzrnActor actor))
      (if (Math|Vector|NotEqual(Vector) (.Location (Math|Transform|BreakTransform sxkjinzhi)) "0, 0, 0" 0.0001)
        (Variables|/Game/BluePrint/LimtSpace/jinzrnActor.jinzrnActor_C|Setpos _asjinzrn_actor sxkjinzhi)))
    (:then_11
      (bind _asban_shou_actor_fan_bao (Utilities|Casting|CastTobanShouActorFanBao actor))
      (if (Math|Vector|NotEqual(Vector) (.Location (Math|Transform|BreakTransform sxkjfanbaobs)) "0, 0, 0" 0.0001)
        (Variables|/Game/BluePrint/FireWork/banShouActorFanBao.banShouActorFanBao_C|Setpos _asban_shou_actor_fan_bao sxkjfanbaobs)))
    (:then_12
      (bind _aszhylweixian_bsblueprint_1 (Utilities|Casting|CastTozhylweixianBSBlueprint1 actor))
      (if (Math|Vector|NotEqual(Vector) (.Location (Math|Transform|BreakTransform zhylweilan)) "0, 0, 0" 0.0001)
        (Variables|/Game/BluePrint/ZongHeYanLian/zhylweixianBSBlueprint1.zhylweixianBSBlueprint1_C|Setpos _aszhylweixian_bsblueprint_1 zhylweilan)))
    (:then_13
      (bind _aszong_he_medkit (Utilities|Casting|CastToZongHeMedkit actor))
      (if (Math|Vector|NotEqual(Vector) (.Location (Math|Transform|BreakTransform zongheMediket)) "0, 0, 0" 0.0001)
        (Variables|/Game/BluePrint/ZongHeYanLian/ZongHeMedkit.ZongHeMedkit_C|Setpos _aszong_he_medkit zongheMediket)))
    (:then_14
      (bind _aszong_he_mang_ban (Utilities|Casting|CastToZongHeMangBan actor))
      (if (Math|Vector|NotEqual(Vector) (.Location (Math|Transform|BreakTransform zonghemangban)) "0, 0, 0" 0.0001)
        (Variables|/Game/BluePrint/ZongHeYanLian/ZongHeMangBan.ZongHeMangBan_C|Setpos _aszong_he_mang_ban zonghemangban)))
    (:then_15
      (bind _asbp_fire_yang_qi_ping (Utilities|Casting|CastToBP_FireYangQiPing actor))
      (if (Math|Vector|NotEqual(Vector) (.Location (Math|Transform|BreakTransform yangqiping)) "0, 0, 0" 0.0001)
        (Variables|/Game/BluePrint/FireWork/BP_FireYangQiPing.BP_FireYangQiPing_C|Setpos _asbp_fire_yang_qi_ping yangqiping)))
    (:then_16
      (bind _asbp_fire_yi_que_ping (Utilities|Casting|CastToBP_FireYiQuePing actor))
      (if (Math|Vector|NotEqual(Vector) (.Location (Math|Transform|BreakTransform yiyueping)) "0, 0, 0" 0.0001)
        (Variables|/Game/BluePrint/FireWork/BP_FireYiQuePing.BP_FireYiQuePing_C|Setpos _asbp_fire_yi_que_ping yiyueping)))
    (:then_17
      (bind _ashanqiang_actor (Utilities|Casting|CastTohanqiangActor actor))
      (if (Math|Vector|NotEqual(Vector) (.Location (Math|Transform|BreakTransform Hanqiang)) "0, 0, 0" 0.0001)
        (Variables|/Game/ceTest/hanqiangActor.hanqiangActor_C|Setpos _ashanqiang_actor Hanqiang)))
    (:then_18
      (bind _aszong_he_fire_extinguisher (Utilities|Casting|CastToZongHeFireExtinguisher actor))
      (if (Math|Vector|NotEqual(Vector) (.Location (Math|Transform|BreakTransform zongheMieHuo)) "0, 0, 0" 0.0001)
        (Variables|/Game/BluePrint/ZongHeYanLian/ZongHeFireExtinguisher.ZongHeFireExtinguisher_C|Setpos _aszong_he_fire_extinguisher zongheMieHuo)))))

(event Custom|UpdatePickUpPos_C
  (params (actor :type Actor%20Object%20Reference) (pos :type Transform))
  (CallFunction|UpdatePickUpPosS actor pos pos pos pos pos pos pos pos pos pos pos pos pos pos pos pos pos pos pos))

(fn ConstructionScript)

(fn GetVRCharacter
  (bind _asmotion_controller_pawn (Utilities|Casting|CastToMotionControllerPawn (Pawn|GetControlledPawn))
    (:then
      (return true _asmotion_controller_pawn))
    (:CastFailed
      (return false 0))))

(fn TeleportFun)