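; VR confirm button for a work-permit drill, pressed through the motion controller's Pickup event.
; State flags select the step: approval, permit issuing with hazard notice, or final sign-off; the first two require a specific character type.
; Paired timelines animate the press along Y, then delayed visibility swaps advance display actors.
; Issuing also sets game-mode flags and reveals a camera; sign-off shows another actor and logs a score of 100.
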(event EventPickup
  (params (AttachTo :type Scene%20Component%20Object%20Reference) (CharacterType :type EcharacterType%20Enum :default "NewEnumerator0"))
  (bind _zonghebtactor9 (Variables|Default|Getzonghebtactor9))
  (bind _zonghetvactor19 (Variables|Default|Getzonghetvactor19))
  (bind _zonghetvactor2 (Variables|Default|Getzonghetvactor2))
  (bind _zonghebtactor2 (Variables|Default|Getzonghebtactor2))
  (bind _zonghetvactor12 (Variables|Default|Getzonghetvactor12))
  (bind _zongheactor6 (Variables|Default|Getzongheactor6))
  (bind _zonghetvactor13 (Variables|Default|Getzonghetvactor13))
  (bind _zonghetvactor20 (Variables|Default|Getzonghetvactor20))
  (if (Variables|Default|GetIsBeforeWork)
    ;[1 1 1] 点击按钮审批成功
    (if (Utilities|Enum|Equal(Enum) CharacterType "NewEnumerator0")
      (bind _offset (Timeline|时间轴_1 Play)
        (:Update
          (Transformation|SetActorLocation (Math|Vector|MakeVector -6757.331543 _offset 102.161179) false false))
        (:Finished
          (bind _offset_2 (Timeline|时间轴_0 PlayFromStart)
            (:Update
              (Transformation|SetActorLocation (Math|Vector|MakeVector -6757.331543 _offset_2 102.161179) false false)
              (Variables|Default|SetIsBeforeWork false)
              (Rendering|SetActorHiddenInGame _zonghetvactor2 true)
              (Rendering|SetActorHiddenInGame (Variables|Default|Getzonghetvactor3) false)
              (Rendering|SetActorHiddenInGame (Variables|Default|Getzonghebtactor1) true)
              (Rendering|SetActorHiddenInGame _zonghebtactor2 false)
              (Utilities|FlowControl|Delay 6.0)
              (Rendering|SetActorHiddenInGame _zonghebtactor2 true)
              (Rendering|SetActorHiddenInGame (Variables|Default|Getzonghebtactor3) false)
              (Rendering|SetActorHiddenInGame _zonghetvactor2 true)
              (Rendering|SetActorHiddenInGame (Variables|Default|Getzonghetvactor4) false)
              (Rendering|SetActorHiddenInGame (Variables|Default|Getzhylfyacrot) false))))))
    (elif (Variables|Default|GetisCanQianFa)
      (if (Utilities|Enum|Equal(Enum) CharacterType "NewEnumerator0")
        (bind _offset_3 (Timeline|时间轴_6 Play)
          (:Update
            (Transformation|SetActorLocation (Math|Vector|MakeVector -6757.331543 _offset_3 102.161179) false false))
          (:Finished
            (bind _offset_4 (Timeline|时间轴_7 PlayFromStart)
              (:Update
                (Transformation|SetActorLocation (Math|Vector|MakeVector -6757.331543 _offset_4 102.161179) false false)
                (Variables|Default|SetisCanQianFa false)
                (Rendering|SetActorHiddenInGame (Variables|Default|Getzonghetvactor11) true)
                (Rendering|SetActorHiddenInGame _zonghetvactor12 false)
                (Rendering|SetActorHiddenInGame (Variables|Default|Getzongheactor5) true)
                (Rendering|SetActorHiddenInGame _zongheactor6 false)
                (Utilities|FlowControl|Delay 3.0)
                (Rendering|SetActorHiddenInGame _zonghetvactor12 true)
                (Rendering|SetActorHiddenInGame _zonghetvactor13 false)
                (Utilities|FlowControl|Delay 3.0)
                (Rendering|SetActorHiddenInGame _zongheactor6 true)
                (Rendering|SetActorHiddenInGame _zonghetvactor13 true)
                (Rendering|SetActorHiddenInGame (Variables|Default|Getzonghetvactor14) false)
                (Rendering|SetActorHiddenInGame (Variables|Default|Getzongheactor7) false)
                (bind _asbp_zong_he_game_mode (Utilities|Casting|CastToBP_ZongHeGameMode (Game|GetGameMode)))
                (Variables|/Game/BluePrint/ZongHeYanLian/BP_ZongHeGameMode.BP_ZongHeGameMode_C|Setzhylwhgz _asbp_zong_he_game_mode true)
                (Variables|Default|SetzhylIsInWork true)
                (bind _asbp_zong_he_game_mode_2 (Utilities|Casting|CastToBP_ZongHeGameMode (Game|GetGameMode)))
                (Variables|/Game/BluePrint/ZongHeYanLian/BP_ZongHeGameMode.BP_ZongHeGameMode_C|SetzhylIsCamera _asbp_zong_he_game_mode_2 true)
                (Rendering|SetActorHiddenInGame (Variables|Default|Getzonghecamera) false))))))
      (elif (Variables|Default|GetisCanQueRen)
        ;[1 1 1] 现场清理完毕后确认并签字
        (bind _offset_5 (Timeline|时间轴_2 Play)
          (:Update
            (Transformation|SetActorLocation (Math|Vector|MakeVector -6757.331543 _offset_5 102.161179) false false))
          (:Finished
            (bind _offset_6 (Timeline|时间轴_3 PlayFromStart)
              (:Update
                (Transformation|SetActorLocation (Math|Vector|MakeVector -6757.331543 _offset_6 102.161179) false false)
                (Variables|Default|SetisCanQueRen false)
                (Rendering|SetActorHiddenInGame (Variables|Default|Getzonghetvactor18) true)
                (Rendering|SetActorHiddenInGame _zonghetvactor19 false)
                (Rendering|SetActorHiddenInGame (Variables|Default|Getzonghebtactor8) true)
                (Rendering|SetActorHiddenInGame _zonghebtactor9 false)
                (Utilities|FlowControl|Delay 5.0)
                (Rendering|SetActorHiddenInGame _zonghebtactor9 true)
                (Rendering|SetActorHiddenInGame (Variables|Default|Getzonghebtactor10) false)
                (Rendering|SetActorHiddenInGame _zonghetvactor19 true)
                (Rendering|SetActorHiddenInGame _zonghetvactor20 false)
                (Utilities|FlowControl|Delay 5.0)
                (Rendering|SetActorHiddenInGame _zonghetvactor20 true)
                (Rendering|SetActorHiddenInGame (Variables|Default|Getzhsxdengji) false)
                (Development|PrintString "scorescore:100" false)))))))))

(event EventDrop)

(fn ConstructionScript)

(fn GetText
  (params (NewParam :type Boolean))
  (if NewParam
    (return "是")
    (else
      (return "否"))))