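; VR-grabbable fire extinguisher for a comprehensive drill (ZongHe) that puts out BP_Fire actors.
; Pickup attaches it to the hand, shows spray if the game mode allows, and starts a timer syncing its transform through MyPlayerController.
; Drop line-traces a ground position, detaches, hides spray and briefly simulates physics.
; Box overlap destroys fires; clearing the last updates game mode flags and swaps staged worker actors on delays.
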(event OnComponentBeginOverlap(Box)
  (params (OverlappedComponent :type Primitive%20Component%20Object%20Reference) (OtherActor :type Actor%20Object%20Reference) (OtherComp :type Primitive%20Component%20Object%20Reference) (OtherBodyIndex :type Integer) (bFromSweep :type Boolean) (SweepResult :type Hit%20Result%20Structure%20%28by%20ref%29))
  (bind _zongheworkactor4 (Variables|Default|Getzongheworkactor4))
  (bind _zongheworkafteractor1 (Variables|Default|Getzongheworkafteractor1))
  ;[1 1 1] 灭火
  (bind _asbp_fire (Utilities|Casting|CastToBP_Fire OtherActor))
  (Actor|DestroyActor _asbp_fire)
  (bind _outactors (Actor|GetAllActorsOfClass "/Game/BluePrint/FireWork/BP_Fire.BP_Fire_C"))
  (if (== (Utilities|Array|Length _outactors) 0)
    (Rendering|SetActorHiddenInGame (Variables|Default|Getzongheworkactor2) true)
    (Rendering|SetActorHiddenInGame _zongheworkactor4 false)
    (bind _asbp_zong_he_game_mode (Utilities|Casting|CastToBP_ZongHeGameMode (Game|GetGameMode)))
    (Variables|/Game/BluePrint/ZongHeYanLian/BP_ZongHeGameMode.BP_ZongHeGameMode_C|SetzhylIsAfterWork _asbp_zong_he_game_mode true)
    (Variables|/Game/BluePrint/ZongHeYanLian/BP_ZongHeGameMode.BP_ZongHeGameMode_C|SetMiehuoQiTeXiao _asbp_zong_he_game_mode false)
    (Utilities|FlowControl|Delay 15.0)
    (Rendering|SetActorHiddenInGame _zongheworkactor4 true)
    (Rendering|SetActorHiddenInGame _zongheworkafteractor1 false)
    (Utilities|FlowControl|Delay 8.0)
    (Rendering|SetActorHiddenInGame _zongheworkafteractor1 true)
    (Rendering|SetActorHiddenInGame (Variables|Default|Getzongheworkafteractor2) false)
    (Rendering|SetActorHiddenInGame (Variables|Default|Getguding1) true)
    (Rendering|SetActorHiddenInGame (Variables|Default|Getguding2) true)))

(event Custom|GetXifu
  (bind _heightpos (Variables|Default|Getheightpos))
  (bind _returnvalue (Transformation|GetWorldLocation _heightpos))
  (bind (_x _y _z) (Math|Vector|BreakVector _returnvalue))
  ;[1 1 1] 吸附地面位置
  (bind _outhit (Collision|LineTraceForObjects (Math|Vector|MakeVector _x _y (+ _z 3e+02)) (Math|Vector|MakeVector _x _y (+ _z -3e+02)) (Utilities|Array|MakeArray "ObjectTypeQuery1") true 0 "None"))
  (bind _asmy_player_controller (Utilities|Casting|CastToMyPlayerController (Game|GetPlayerController 0)))
  (Default|UpdatePickUpPosC _asmy_player_controller self (Math|Transform|MakeTransform (Math|Vector|MakeVector (.X (Math|Vector|BreakVector (.Location (Collision|BreakHitResult _outhit)))) (.Y (Math|Vector|BreakVector (.Location (Collision|BreakHitResult _outhit)))) (+ (.Z (Math|Vector|BreakVector (.Location (Collision|BreakHitResult _outhit)))) 1.0)) (Math|Rotator|MakeRotator 0.0 0.0 (.yaw (Transformation|GetWorldRotation (Variables|Debug|GetStaticMeshComponent)))) (Transformation|GetWorldScale (Variables|Default|GetHeightpos)))))

(event Custom|UpdatePos_C
  (bind _self self)
  (bind _hand (Variables|Default|Gethand))
  (bind _scene (Variables|Default|GetScene))
  (bind _staticmesh (Variables|Default|GetStaticMesh))
  (bind _returnvalue (Transformation|GetWorldTransform _hand))
  (bind _returnvalue_2 (Transformation|GetWorldLocation _staticmesh))
  (bind _returnvalue_3 (Transformation|GetWorldLocation _scene))
  (bind _returnvalue_4 (- _returnvalue_2 _returnvalue_3))
  (bind (_roll _pitch _yaw) (Math|Rotator|BreakRotator (.rotation _returnvalue)))
  (bind _returnvalue_5 (+ (.location _returnvalue) _returnvalue_4))
  ;[1 1 1] 同步灭火器位置
  (bind _asmy_player_controller (Utilities|Casting|CastToMyPlayerController (Game|GetPlayerController 0)))
  (if (< (.Y (Math|Vector|BreakVector (.scale _returnvalue))) 0.0)
    (Default|UpdatePickUpPosC _asmy_player_controller _self (Math|Transform|MakeTransform _returnvalue_5 (Math|Rotator|MakeRotator (+ _roll 9e+01) _pitch _yaw) "1,1,1"))
    (else
      (Default|UpdatePickUpPosC _asmy_player_controller _self (Math|Transform|MakeTransform _returnvalue_5 (Math|Rotator|MakeRotator (- _roll 9e+01) _pitch _yaw) "1,1,1")))))

(event Custom|SetPickUp_S
  (params (IsPickUp :type Boolean))
  ;[1 1 1] 设置灭火器是否被抓状态
  (Variables|Default|SetIsPickUp IsPickUp))

(event EventPickup
  (params (AttachTo :type Scene%20Component%20Object%20Reference) (CharacterType :type EcharacterType%20Enum :default "NewEnumerator0"))
  (Variables|Default|Sethand AttachTo)
  (Utilities|FlowControl|Sequence
    (:then_0
      (CallFunction|SetPickUpS false))
    (:then_1
      (Transformation|AttachComponentToComponent (VehicleSound|GetRootComponent) AttachTo "None" "KeepWorld" "KeepWorld" "KeepWorld" false)
      (bind _asbp_zong_he_game_mode (Utilities|Casting|CastToBP_ZongHeGameMode (Game|GetGameMode)))
      (if (Variables|/Game/BluePrint/ZongHeYanLian/BP_ZongHeGameMode.BP_ZongHeGameMode_C|GetMiehuoQiTeXiao _asbp_zong_he_game_mode)
        (Rendering|SetVisibility (Variables|Default|GetParticleSystem) true false)))
    (:then_2
      ;[1 1 1] 心跳同步
      (Utilities|Time|SetTimerbyFunctionName 0 "UpdatePos" 0.05 true))))

(event EventDrop
  (bind _staticmeshcomponent (Variables|Debug|GetStaticMeshComponent))
  (Utilities|FlowControl|Sequence
    (:then_0
      ;[1 1 1] 设置灭火器不被抓
      (CallFunction|SetPickUpS false))
    (:then_1
      ;[1 1 1] 取消心跳同步
      (Utilities|Time|ClearTimerbyFunctionName 0 "UpdatePos"))
    (:then_2
      ;[1 1 1] 计算吸附地面位置
      (CallFunction|GetXifu))
    (:then_3
      (Transformation|DetachFromActor "KeepWorld" "KeepWorld" "KeepWorld")
      (Rendering|SetVisibility (Variables|Default|GetParticleSystem) false false)
      (Physics|SetSimulatePhysics _staticmeshcomponent true)
      (Utilities|FlowControl|Delay 1.0)
      (Physics|SetSimulatePhysics _staticmeshcomponent false))))

(fn ConstructionScript)

(fn OnRepPos
  (bind _pos (Variables|Default|Getpos))
  (if (Math|Vector|NotEqual(Vector) (.Location (Math|Transform|BreakTransform _pos)) "0, 0, 0" 0.1)
    (Transformation|SetWorldTransform (Variables|Debug|GetStaticMeshComponent) _pos false false)
    (Components|Activation|SetActive (Variables|Default|GetParticleSystem) true false)))

(fn UpdatePos
  (CallFunction|UpdatePosC))