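; Bottle UI actor for the comprehensive drill (ZongHeYanLian), covering removal of oxygen and acetylene cylinders.
; Once both cylinder flags are set, it hides itself and checks garbage clearing, valve, gas detection and safety equipment flags on BP_ZongHeGameMode.
; If all pass, it swaps scene actor visibility and sets the game mode's ZhylZYZ flag after a short delay.
; Otherwise it reveals three other actors, including a score actor.
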(event Custom|BottleUIyichu
  (if (and (Variables|Default|GetzhylIsYangQiPing) (Variables|Default|GetzhylIsYiQuePing))
    (Utilities|Casting|CastToBP_ZongHeGameMode (Game|GetGameMode))
    (Rendering|SetActorHiddenInGame self true)
    (CallFunction|Cheackzhyl)))

(event Custom|cheackzhyl
  (bind _asbp_zong_he_game_mode (Utilities|Casting|CastToBP_ZongHeGameMode (Game|GetGameMode)))
  (if (Math|Boolean|ANDBoolean (Variables|/Game/BluePrint/ZongHeYanLian/BP_ZongHeGameMode.BP_ZongHeGameMode_C|GetZHYLIsClearGarbage _asbp_zong_he_game_mode) (Variables|/Game/BluePrint/ZongHeYanLian/BP_ZongHeGameMode.BP_ZongHeGameMode_C|GetzhylFaMenUI _asbp_zong_he_game_mode) (Variables|/Game/BluePrint/ZongHeYanLian/BP_ZongHeGameMode.BP_ZongHeGameMode_C|GetzhyliSGasdetection _asbp_zong_he_game_mode) (Variables|/Game/BluePrint/ZongHeYanLian/BP_ZongHeGameMode.BP_ZongHeGameMode_C|GetzhylIsAnQuanQiCai _asbp_zong_he_game_mode))
    (Rendering|SetActorHiddenInGame (Variables|Default|Getzongheactor4) true)
    (Rendering|SetActorHiddenInGame (Variables|Default|Getzongheactor5) false)
    (Rendering|SetActorHiddenInGame (Variables|Default|Getzonghetvactor7) true)
    (Rendering|SetActorHiddenInGame (Variables|Default|Getzonghetvactor8) false)
    (Utilities|FlowControl|Delay 3.0)
    (Variables|/Game/BluePrint/ZongHeYanLian/BP_ZongHeGameMode.BP_ZongHeGameMode_C|SetzhylZYZ _asbp_zong_he_game_mode true)
    (else
      (Rendering|SetActorHiddenInGame (Variables|Default|Getshibatishi2222) false)
      (Rendering|SetActorHiddenInGame (Variables|Default|Getzhsxscore) false)
      (Rendering|SetActorHiddenInGame (Variables|Default|Getzyqbzylactor) false))))

(fn ConstructionScript)