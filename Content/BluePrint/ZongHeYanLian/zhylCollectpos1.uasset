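; Collection point for the comprehensive drill (ZongHeYanLian) that checks whether six tools and safety items have been brought back after work.
; Box overlaps, active only while the GameMode's ZhylIsAfterWork is set, latch a flag per item class: extinguisher, medkit, rope, blind plate, plate sign, searchlight.
; Once all flags are set, it hides the after-work actor, then after a delay enables UI confirmation and swaps the button and TV actors' visibility.
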(event OnComponentBeginOverlap(Box)
  (params (OverlappedComponent :type Primitive%20Component%20Object%20Reference) (OtherActor :type Actor%20Object%20Reference) (OtherComp :type Primitive%20Component%20Object%20Reference) (OtherBodyIndex :type Integer) (bFromSweep :type Boolean) (SweepResult :type Hit%20Result%20Structure%20%28by%20ref%29))
  (bind _asbp_zong_he_game_mode (Utilities|Casting|CastToBP_ZongHeGameMode (Game|GetGameMode)))
  (if (Variables|/Game/BluePrint/ZongHeYanLian/BP_ZongHeGameMode.BP_ZongHeGameMode_C|GetzhylIsAfterWork _asbp_zong_he_game_mode)
    (Utilities|FlowControl|Sequence
      (:then_0
        (Utilities|Casting|CastToMedkit OtherActor)
        (Variables|Default|SetHasMedKit true)
        (CallFunction|ZhylCheckClear))
      (:then_1
        (Utilities|Casting|CastToRoop OtherActor)
        (Variables|Default|SetHasRoop true)
        (CallFunction|ZhylCheckClear))
      (:then_2
        (Utilities|Casting|CastToZongHeFireExtinguisher OtherActor)
        (Variables|Default|SetHasFireExting true)
        (CallFunction|ZhylCheckClear))
      (:then_3
        (Utilities|Casting|CastTozhylMangBanBiaoZhiActorPos2 OtherActor)
        (Variables|Default|SetHasMangBanBS true)
        (CallFunction|ZhylCheckClear))
      (:then_4
        (Utilities|Casting|CastToZongHeMangBan OtherActor)
        (Variables|Default|SetHasMangBan true)
        (CallFunction|ZhylCheckClear))
      (:then_5
        (Utilities|Casting|CastTotanzhaodeng OtherActor)
        (Variables|Default|SetHasTanzhaodeng true)
        (CallFunction|ZhylCheckClear)))))

(event Custom|zhylCheckClear
  (Utilities|Casting|CastToBP_ZongHeGameMode (Game|GetGameMode))
  (if (Math|Boolean|ANDBoolean (Variables|Default|GetHasFireExting) (Variables|Default|GetHasMedKit) (Variables|Default|GetHasRoop) (Variables|Default|GetHasMangBan) (Variables|Default|GetHasMangBanBS) (Variables|Default|GetHasTanzhaodeng))
    (Rendering|SetActorHiddenInGame (Variables|Default|Getzongheworkafteractor2) true)
    (Utilities|FlowControl|Delay 2.0)
    (Rendering|SetActorHiddenInGame (Variables|Default|Getzonghebtactor8) false)
    (Variables|/Game/BluePrint/ZongHeYanLian/BP_ZongHeConfirmButton.BP_ZongHeConfirmButton_C|SetisCanQueRen (Variables|Default|GetzongheConfirmUI) true)
    (Rendering|SetActorHiddenInGame (Variables|Default|Getzonghetvactor17) true)
    (Rendering|SetActorHiddenInGame (Variables|Default|Getzonghetvactor18) false)))

(fn ConstructionScript)