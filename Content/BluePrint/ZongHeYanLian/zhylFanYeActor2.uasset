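; Page-turn (FanYe) actor for the ZongHeYanLian scenario: each Pickup advances a sequence of screen actors by toggling visibility.
; Chained one-shot booleans pick the step across three runs, the latter two unlocked by BP_ZongHeGameMode flags.
; Each step's timeline slides the actor along Y and, on Update, swaps screens, usually detaches via Drop and arms the next step.
; Run endings swap or hide other actors or enable ZhylConfirmBT; alternate timeline loops are unwired.
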(event EventPickup
  (params (AttachTo :type Scene%20Component%20Object%20Reference) (CharacterType :type EcharacterType%20Enum :default "NewEnumerator0"))
  (if (Variables|Default|GetzhylIsfirstFY)
    (Variables|Default|SetzhylIsfirstFY false)
    (bind _offset (Timeline|时间轴_0 Play)
      (:Update
        (Transformation|SetActorLocation (Math|Vector|MakeVector -7113.035156 _offset 76.260162) false false)
        (Rendering|SetActorHiddenInGame (Variables|Default|GetzonghetvActor4) true)
        (Rendering|SetActorHiddenInGame (Variables|Default|Getzonghetvactor5) false)
        (CallFunction|Drop)
        (Variables|Default|SetzhylIsSecondFY true)))
    (elif (Variables|Default|GetzhylIsSecondFY)
      (Variables|Default|SetzhylIsSecondFY false)
      (bind _offset_2 (Timeline|时间轴_2 Play)
        (:Update
          (Transformation|SetActorLocation (Math|Vector|MakeVector -7113.035156 _offset_2 76.260162) false false)
          (Rendering|SetActorHiddenInGame (Variables|Default|Getzonghetvactor5) true)
          (Rendering|SetActorHiddenInGame (Variables|Default|Getzonghetvactor6) false)
          (CallFunction|Drop)
          (Variables|Default|SetzhylThirdFY true)))
      (elif (Variables|Default|GetzhylThirdFY)
        (Variables|Default|SetzhylThirdFY false)
        (bind _offset_3 (Timeline|时间轴_4 Play)
          (:Update
            (Transformation|SetActorLocation (Math|Vector|MakeVector -7113.035156 _offset_3 76.260162) false false)
            (Rendering|SetActorHiddenInGame (Variables|Default|Getzonghetvactor6) true)
            (Rendering|SetActorHiddenInGame (Variables|Default|Getzonghetvactor7) false)
            (CallFunction|Drop)
            (Utilities|FlowControl|Delay 2.5)
            (Rendering|SetActorHiddenInGame (Variables|Default|Getzonghebtactor3) true)
            (Rendering|SetActorHiddenInGame (Variables|Default|Getzonghebtactor4) false)))
        (else
          (bind _asbp_zong_he_game_mode (Utilities|Casting|CastToBP_ZongHeGameMode (Game|GetGameMode)))
          (if (Variables|/Game/BluePrint/ZongHeYanLian/BP_ZongHeGameMode.BP_ZongHeGameMode_C|GetzhylZYZ _asbp_zong_he_game_mode)
            (Variables|/Game/BluePrint/ZongHeYanLian/BP_ZongHeGameMode.BP_ZongHeGameMode_C|SetzhylZYZ _asbp_zong_he_game_mode false)
            (bind _offset_4 (Timeline|时间轴_6 Play)
              (:Update
                (Transformation|SetActorLocation (Math|Vector|MakeVector -7113.035156 _offset_4 76.260162) false false)
                (Rendering|SetActorHiddenInGame (Variables|Default|Getzonghetvactor8) true)
                (Rendering|SetActorHiddenInGame (Variables|Default|Getzonghetvactor9) false)
                (CallFunction|Drop)
                (Variables|Default|Setzhylzyz01 true)))
            (elif (Variables|Default|Getzhylzyz01)
              (Variables|Default|Setzhylzyz01 false)
              (bind _offset_5 (Timeline|时间轴_8 Play)
                (:Update
                  (Transformation|SetActorLocation (Math|Vector|MakeVector -7113.035156 _offset_5 76.260162) false false)
                  (Rendering|SetActorHiddenInGame (Variables|Default|Getzonghetvactor9) true)
                  (Rendering|SetActorHiddenInGame (Variables|Default|Getzongheactor10) false)
                  (CallFunction|Drop)
                  (Variables|Default|Setzhylzyz02 true)))
              (elif (Variables|Default|Getzhylzyz02)
                (Variables|Default|Setzhylzyz02 false)
                (bind _offset_6 (Timeline|时间轴_10 Play)
                  (:Update
                    (Transformation|SetActorLocation (Math|Vector|MakeVector -7113.035156 _offset_6 76.260162) false false)
                    (Rendering|SetActorHiddenInGame (Variables|Default|Getzongheactor10) true)
                    (Rendering|SetActorHiddenInGame (Variables|Default|Getzonghetvactor11) false)
                    (CallFunction|Drop)
                    (Variables|/Game/BluePrint/ZongHeYanLian/BP_ZongHeConfirmButton.BP_ZongHeConfirmButton_C|SetisCanQianFa (Variables|Default|GetzhylConfirmBT) true)))
                (else
                  (bind _asbp_zong_he_game_mode_2 (Utilities|Casting|CastToBP_ZongHeGameMode (Game|GetGameMode)))
                  (if (Variables|/Game/BluePrint/ZongHeYanLian/BP_ZongHeGameMode.BP_ZongHeGameMode_C|Getzhylwhgz _asbp_zong_he_game_mode_2)
                    (Variables|/Game/BluePrint/ZongHeYanLian/BP_ZongHeGameMode.BP_ZongHeGameMode_C|Setzhylwhgz _asbp_zong_he_game_mode_2 false)
                    (bind _offset_7 (Timeline|时间轴_12 Play)
                      (:Update
                        (Transformation|SetActorLocation (Math|Vector|MakeVector -7113.035156 _offset_7 76.260162) false false)
                        (Rendering|SetActorHiddenInGame (Variables|Default|Getzonghetvactor14) true)
                        (Rendering|SetActorHiddenInGame (Variables|Default|Getzonghetvactor15) false)
                        (CallFunction|Drop)
                        (Variables|Default|Setzhylwhgz01 true)))
                    (elif (Variables|Default|Getzhylwhgz01)
                      (Variables|Default|Setzhylwhgz01 false)
                      (bind _offset_8 (Timeline|时间轴_14 Play)
                        (:Update
                          (Transformation|SetActorLocation (Math|Vector|MakeVector -7113.035156 _offset_8 76.260162) false false)
                          (Rendering|SetActorHiddenInGame (Variables|Default|Getzonghetvactor15) true)
                          (Rendering|SetActorHiddenInGame (Variables|Default|Getzonghetvactor16) false)
                          (CallFunction|Drop)
                          (Variables|Default|Setzhylwhgz02 true)))
                      (elif (Variables|Default|Getzhylwhgz02)
                        (Variables|Default|Setzhylwhgz02 false)
                        (bind _offset_9 (Timeline|时间轴_16 Play)
                          (:Update
                            (Transformation|SetActorLocation (Math|Vector|MakeVector -7113.035156 _offset_9 76.260162) false false)
                            (Rendering|SetActorHiddenInGame (Variables|Default|Getzonghetvactor16) true)
                            (Rendering|SetActorHiddenInGame (Variables|Default|Getzonghetvactor17) false)
                            (Utilities|FlowControl|Delay 3.0)
                            (Rendering|SetActorHiddenInGame (Variables|Default|Getzongheactor7) true)))))))))))))))

(event EventDrop
  (Utilities|Casting|CastToBP_ZongHeGameMode (Game|GetGameMode))
  (Transformation|DetachFromActor "KeepWorld" "KeepWorld" "KeepWorld"))

(fn ConstructionScript)