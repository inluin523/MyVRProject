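; Grabbable actor for the ZongHeYanLian mode, apparently a position marker for a blind-plate sign (MangBanBiaoZhi), hidden in game on BeginPlay.
; Pickup disables physics on its static mesh and attaches the root to the supplied component, keeping world transform.
; Drop re-enables physics and detaches it.
; Both require BP_ZongHeGameMode, though the cast result is unused and the following branch is always true.
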(event EventBeginPlay
  (Rendering|SetActorHiddenInGame true))

(event EventPickup
  (params (AttachTo :type Scene%20Component%20Object%20Reference) (CharacterType :type EcharacterType%20Enum :default "NewEnumerator0"))
  (Utilities|Casting|CastToBP_ZongHeGameMode (Game|GetGameMode))
  (if true
    (Physics|SetSimulatePhysics (Variables|Debug|GetStaticMeshComponent) false)
    (Transformation|AttachComponentToComponent (VehicleSound|GetRootComponent) AttachTo "None" "KeepWorld" "KeepWorld" "KeepWorld" false)))

(event EventDrop
  (Utilities|Casting|CastToBP_ZongHeGameMode (Game|GetGameMode))
  (if true
    (Physics|SetSimulatePhysics (Variables|Debug|GetStaticMeshComponent) true)
    (Transformation|DetachFromActor "KeepWorld" "KeepWorld" "KeepWorld")))

(fn ConstructionScript)