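; Actor for the comprehensive drill (ZongHeYanLian) whose widget serves as a safety-equipment slogan.
; The custom event aqcqyc casts to BP_ZongHeGameMode and checks whether the safety-equipment stage is still incomplete.
; When the rope, fire extinguisher, medical and searchlight flags are all true, it hides the widget and sets the game mode's ZhylIsAnQuanQiCai flag.
; BeginPlay, overlap and construction logic are empty.
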(event Custom|aqcqyc
  (bind _asbp_zong_he_game_mode (Utilities|Casting|CastToBP_ZongHeGameMode (Game|GetGameMode)))
  (if (not (Variables|/Game/BluePrint/ZongHeYanLian/BP_ZongHeGameMode.BP_ZongHeGameMode_C|GetzhylIsAnQuanQiCai _asbp_zong_he_game_mode))
    (if (Math|Boolean|ANDBoolean (Variables|Default|GetzhylIsRoopCorrect) (Variables|Default|Getzhylmiehuoqi) (Variables|Default|GetzhylIsMedicalCorrect) (Variables|Default|GetzhylisTanzhaodeng))
      (Rendering|SetVisibility (Variables|Default|GetWidget) false false)
      (Variables|/Game/BluePrint/ZongHeYanLian/BP_ZongHeGameMode.BP_ZongHeGameMode_C|SetzhylIsAnQuanQiCai _asbp_zong_he_game_mode true))))

(event EventBeginPlay)

(event Collision|EventActorBeginOverlap
  (params (OtherActor :type Actor%20Object%20Reference)))

(fn ConstructionScript)