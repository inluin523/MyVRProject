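; Valve (famen) actor for the comprehensive drill (ZongHeYanLian) that validates a valve operation step when its famenUIyichu event runs.
; While the GameMode's ZhylFaMenUI flag is unset, it checks the sign, blind plate, tap rotation and wrench states.
; Success sets the flag, calls Zhylmmss, then uses delays to hide the widget and temporarily show a hint actor.
; Failure reveals the failure, score and Fmczyw actors.
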(event Custom|famenUIyichu
  (bind _zhsxqitishiactorr (Variables|Default|Getzhsxqitishiactorr))
  (bind _asbp_zong_he_game_mode (Utilities|Casting|CastToBP_ZongHeGameMode (Game|GetGameMode)))
  (if (not (Variables|/Game/BluePrint/ZongHeYanLian/BP_ZongHeGameMode.BP_ZongHeGameMode_C|GetzhylFaMenUI _asbp_zong_he_game_mode))
    (if (Math|Boolean|ANDBoolean (Variables|Default|Getisbiaoshi) (Variables|Default|Getismangban) (Variables|/Game/ceTest/Tap.Tap_C|GetisXuanZhuan (Variables|Default|GetdhzyTap)) (Variables|/Game/BluePrint/ZongHeYanLian/zhylguandaoActor1.zhylguandaoActor1_C|GetISbanshou (Variables|Default|Getisbansouooo)))
      (Variables|/Game/BluePrint/ZongHeYanLian/BP_ZongHeGameMode.BP_ZongHeGameMode_C|SetzhylFaMenUI _asbp_zong_he_game_mode true)
      (Default|Zhylmmss (Variables|Default|Getzhylmbs))
      (Utilities|FlowControl|Delay 2.0)
      (Rendering|SetVisibility (Variables|Default|GetWidget) false false)
      (Utilities|FlowControl|Delay 2.0)
      (Rendering|SetActorHiddenInGame _zhsxqitishiactorr false)
      (Utilities|FlowControl|Delay 6e+01)
      (Rendering|SetActorHiddenInGame _zhsxqitishiactorr true)
      (else
        (Rendering|SetActorHiddenInGame (Variables|Default|Getshibaiactor1111) false)
        (Rendering|SetActorHiddenInGame (Variables|Default|Getzhsxscore) false)
        (Rendering|SetActorHiddenInGame (Variables|Default|Getfmczywactor) false)))))

(fn ConstructionScript)