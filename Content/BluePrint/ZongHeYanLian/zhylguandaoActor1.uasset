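; Pipeline actor in the comprehensive drill (ZongHeYanLian) that detects blind plates (MangBan), their signs and wrenches entering its box.
; An overlapping sign is destroyed, the actor reveals its preset sign, sets Isbiaoshi on IsfamenOperate and calls FamenUIyichu the first time.
; A blind plate sets Ismangban on IsfamenOperate, while a wrench sets the local ISbanshou flag.
; Overlaps are handled only under BP_ZongHeGameMode.
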(event OnComponentBeginOverlap(box)
  (params (OverlappedComponent :type Primitive%20Component%20Object%20Reference) (OtherActor :type Actor%20Object%20Reference) (OtherComp :type Primitive%20Component%20Object%20Reference) (OtherBodyIndex :type Integer) (bFromSweep :type Boolean) (SweepResult :type Hit%20Result%20Structure%20%28by%20ref%29))
  (bind _isfamenoperate (Variables|Default|GetIsfamenOperate))
  (Utilities|Casting|CastToBP_ZongHeGameMode (Game|GetGameMode))
  (bind _aszong_he_mang_ban_biao_zhi_actor (Utilities|Casting|CastToZongHeMangBanBiaoZhiActor OtherActor)
    (:then
      (Actor|DestroyActor _aszong_he_mang_ban_biao_zhi_actor)
      (Rendering|SetActorHiddenInGame (Variables|Default|GetmangbanbiaoshiActorpos1) false)
      (if (not (Variables|/Game/BluePrint/ZongHeYanLian/zhylfamenActor1.zhylfamenActor1_C|Getisbiaoshi _isfamenoperate))
        (Variables|/Game/BluePrint/ZongHeYanLian/zhylfamenActor1.zhylfamenActor1_C|Setisbiaoshi _isfamenoperate true)
        (Default|FamenUIyichu _isfamenoperate)))
    (:CastFailed
      (Utilities|Casting|CastToZongHeMangBan OtherActor
        (:then
          (if (not (Variables|/Game/BluePrint/ZongHeYanLian/zhylfamenActor1.zhylfamenActor1_C|Getismangban _isfamenoperate))
            (Variables|/Game/BluePrint/ZongHeYanLian/zhylfamenActor1.zhylfamenActor1_C|Setismangban _isfamenoperate true)))
        (:CastFailed
          (Utilities|Casting|CastTobanShouActor OtherActor)
          (Variables|Default|SetISbanshou true))))))

(event EventBeginPlay)

(event Collision|EventActorBeginOverlap
  (params (OtherActor :type Actor%20Object%20Reference)))

(event EventTick
  (params (DeltaSeconds :type Float%20%28single-precision%29)))

(fn ConstructionScript)