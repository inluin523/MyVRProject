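; Gas detection checkpoint actor for the comprehensive drill (ZongHeYanLian) level, with an additional trigger for placing a "jinzhi" (prohibition) object.
; When a motion controller with a visible gas detector first overlaps the Sphere, it writes fixed readings to the detector's screen widget, sets the GameMode's completion flag and calls Gasuiyichu on GasDetectionUIyc.
; When a jinzrnActor overlaps the Box, that actor is destroyed and the hidden Jinzhiactorpos is shown in its place.
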(event OnComponentBeginOverlap(Sphere)
  (params (OverlappedComponent :type Primitive%20Component%20Object%20Reference) (OtherActor :type Actor%20Object%20Reference) (OtherComp :type Primitive%20Component%20Object%20Reference) (OtherBodyIndex :type Integer) (bFromSweep :type Boolean) (SweepResult :type Hit%20Result%20Structure%20%28by%20ref%29))
  (bind _asbp_motion_controller (Utilities|Casting|CastToBP_MotionController OtherActor))
  (bind _asbp_zong_he_game_mode (Utilities|Casting|CastToBP_ZongHeGameMode (Game|GetGameMode)))
  (if (not (Variables|/Game/BluePrint/ZongHeYanLian/BP_ZongHeGameMode.BP_ZongHeGameMode_C|GetzhyliSGasdetection _asbp_zong_he_game_mode))
    (if (Rendering|IsVisible (Variables|/Game/BluePrint/BP_MotionController.BP_MotionController_C|GetGasDetection _asbp_motion_controller))
      (bind _asgas_detection_ui (Utilities|Casting|CastToGasDetectionUI (UserInterface|GetUserWidgetObject (Variables|/Game/BluePrint/BP_MotionController.BP_MotionController_C|GetScreen _asbp_motion_controller))))
      (Variables|/Game/UI/FireWork/GasDetectionUI.GasDetectionUI_C|SetExplodeLimitText _asgas_detection_ui "5%")
      (Variables|/Game/UI/FireWork/GasDetectionUI.GasDetectionUI_C|SetGasDetectionText _asgas_detection_ui "0.3%")
      (Variables|/Game/BluePrint/ZongHeYanLian/BP_ZongHeGameMode.BP_ZongHeGameMode_C|SetzhyliSGasdetection _asbp_zong_he_game_mode true)
      (Default|Gasuiyichu (Variables|Default|GetGasDetectionUIyc)))))

(event OnComponentBeginOverlap(Box)
  (params (OverlappedComponent :type Primitive%20Component%20Object%20Reference) (OtherActor :type Actor%20Object%20Reference) (OtherComp :type Primitive%20Component%20Object%20Reference) (OtherBodyIndex :type Integer) (bFromSweep :type Boolean) (SweepResult :type Hit%20Result%20Structure%20%28by%20ref%29))
  (Utilities|Casting|CastToBP_ZongHeGameMode (Game|GetGameMode))
  (bind _asjinzrn_actor (Utilities|Casting|CastTojinzrnActor OtherActor))
  (Actor|DestroyActor _asjinzrn_actor)
  (Rendering|SetActorHiddenInGame (Variables|Default|Getjinzhiactorpos) false))

(fn ConstructionScript)