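; Danger warning sign actor for the comprehensive drill (ZongHeYanLian) that handles a one-time safe-distance step.
; When a zhylweixianBSBlueprint1 actor overlaps its Box, it sets the ZhylIsAnQuanJuLi flag so the step does not repeat.
; It then hides that actor's widget, swaps the first TV actor for the second, and reveals the JingJieUI actors and QuerenBT confirm button.
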(event OnComponentBeginOverlap(Box)
  (params (OverlappedComponent :type Primitive%20Component%20Object%20Reference) (OtherActor :type Actor%20Object%20Reference) (OtherComp :type Primitive%20Component%20Object%20Reference) (OtherBodyIndex :type Integer) (bFromSweep :type Boolean) (SweepResult :type Hit%20Result%20Structure%20%28by%20ref%29))
  (Utilities|Casting|CastToBP_ZongHeGameMode (Game|GetGameMode))
  (if (not (Variables|Default|GetzhylIsAnQuanJuLi))
    (bind _aszhylweixian_bsblueprint_1 (Utilities|Casting|CastTozhylweixianBSBlueprint1 OtherActor))
    (Variables|Default|SetzhylIsAnQuanJuLi true)
    (Rendering|SetVisibility (Variables|/Game/BluePrint/ZongHeYanLian/zhylweixianBSBlueprint1.zhylweixianBSBlueprint1_C|GetWidget _aszhylweixian_bsblueprint_1) false false)
    (Rendering|SetActorHiddenInGame (Variables|Default|GetzongheTVactor1) true)
    (Rendering|SetActorHiddenInGame (Variables|Default|GetzonghetvActor2) false)
    (for _array_element (Variables|Default|GetjingJieUI)
      (Rendering|SetActorHiddenInGame _array_element false)
      (Rendering|SetActorHiddenInGame (Variables|Default|GetquerenBT) false))))

(fn ConstructionScript)