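; Work position trigger for the ZongHeYanLian scenario that runs a welding-gun (hanqiang) task when that actor overlaps its box.
; A seeded random bool picks one of two outcomes, both staged with delays and actor visibility swaps.
; False spawns fires at preset points and sets the extinguisher-effect flag; true steps through timed work and after-work displays.
; Both flag work as finished on BP_ZongHeGameMode and call Zhylmmsyk.
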(event OnComponentBeginOverlap(Box)
  (params (OverlappedComponent :type Primitive%20Component%20Object%20Reference) (OtherActor :type Actor%20Object%20Reference) (OtherComp :type Primitive%20Component%20Object%20Reference) (OtherBodyIndex :type Integer) (bFromSweep :type Boolean) (SweepResult :type Hit%20Result%20Structure%20%28by%20ref%29))
  (bind _zongheactorsx1 (Variables|Default|Getzongheactorsx1))
  (bind _zongeheworkafteractor1 (Variables|Default|Getzongeheworkafteractor1))
  (if (Math|Boolean|Equal(Boolean) (Math|Random|RandomBoolfromStream (Variables|Default|Getrandom111)) false)
    (Utilities|Casting|CastTohanqiangActor OtherActor)
    ;[1 1 1] 进行作业
    (Utilities|FlowControl|Delay 5.0)
    (Rendering|SetActorHiddenInGame (Variables|Default|Gethanqiang) true)
    (Rendering|SetActorHiddenInGame (Variables|Default|Getzongheactor1) true)
    (Rendering|SetActorHiddenInGame (Variables|Default|Getzongheactor3) false)
    (Rendering|SetActorHiddenInGame (Variables|Default|GetworkUI) true)
    (for _array_element (Variables|Default|GetFireExplodePos)
      (Game|SpawnActorfromClass "/Game/BluePrint/FireWork/BP_Fire.BP_Fire_C" (Transformation|GetActorTransform _array_element) "Undefined" 0 0)
      (bind _asbp_zong_he_game_mode (Utilities|Casting|CastToBP_ZongHeGameMode (Game|GetGameMode)))
      (Variables|/Game/BluePrint/ZongHeYanLian/BP_ZongHeGameMode.BP_ZongHeGameMode_C|SetMiehuoQiTeXiao _asbp_zong_he_game_mode true)
      (Variables|/Game/BluePrint/ZongHeYanLian/BP_ZongHeGameMode.BP_ZongHeGameMode_C|SetzhylIsAfterWork _asbp_zong_he_game_mode true)
      (Default|Zhylmmsyk (Variables|Default|Getmmsyk))
      (Rendering|SetActorHiddenInGame (Variables|Default|Getgudingactor) true)
      (Rendering|SetActorHiddenInGame (Variables|Default|Getguding222) true))
    (else
      (Utilities|Casting|CastTohanqiangActor OtherActor)
      (Utilities|FlowControl|Delay 5.0)
      (Rendering|SetActorHiddenInGame (Variables|Default|Gethanqiang) true)
      (Rendering|SetActorHiddenInGame (Variables|Default|Getzongheactor1) true)
      (Rendering|SetActorHiddenInGame (Variables|Default|Getzongheactor2) false)
      (Rendering|SetActorHiddenInGame (Variables|Default|GetworkUI) true)
      (Rendering|SetActorHiddenInGame _zongheactorsx1 false)
      (Utilities|FlowControl|Delay 15.0)
      (Rendering|SetActorHiddenInGame (Variables|Default|Getzongheactor2) true)
      (Utilities|FlowControl|Delay 5.0)
      (Rendering|SetActorHiddenInGame _zongheactorsx1 true)
      (Rendering|SetActorHiddenInGame _zongeheworkafteractor1 false)
      (Utilities|FlowControl|Delay 1e+01)
      (Rendering|SetActorHiddenInGame _zongeheworkafteractor1 true)
      (Rendering|SetActorHiddenInGame (Variables|Default|Getzongheworkaftreractor2) false)
      (Utilities|FlowControl|Delay 3.0)
      (Default|Zhylmmsyk (Variables|Default|Getmmsyk))
      (Rendering|SetActorHiddenInGame (Variables|Default|Getgudingactor) true)
      (Rendering|SetActorHiddenInGame (Variables|Default|Getguding222) true)
      (bind _asbp_zong_he_game_mode_2 (Utilities|Casting|CastToBP_ZongHeGameMode (Game|GetGameMode)))
      (Variables|/Game/BluePrint/ZongHeYanLian/BP_ZongHeGameMode.BP_ZongHeGameMode_C|SetzhylIsAfterWork _asbp_zong_he_game_mode_2 true))))

(fn ConstructionScript)