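; Detection actor that checks gas bottles (apparently acetylene and oxygen) are returned after work, in the fire or comprehensive (ZongHe) game mode.
; When the after-work flag is set, Box overlaps set per-bottle flags; both together mark the mode's bottle flag and run that mode's clear check.
; Both bottle casts target fuzhiBP_FireYangQiPing1, so the oxygen branch, reached only when the first fails, cannot succeed as written.
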(event OnComponentBeginOverlap(Box)
  (params (OverlappedComponent :type Primitive%20Component%20Object%20Reference) (OtherActor :type Actor%20Object%20Reference) (OtherComp :type Primitive%20Component%20Object%20Reference) (OtherBodyIndex :type Integer) (bFromSweep :type Boolean) (SweepResult :type Hit%20Result%20Structure%20%28by%20ref%29))
  (bind _asfire_game_mode (Utilities|Casting|CastToFireGameMode (Game|GetGameMode))
    (:then
      (if (Variables|/Game/BluePrint/FireGameMode.FireGameMode_C|GetisAfterWork _asfire_game_mode)
        (Utilities|Casting|CastTofuzhiBP_FireYangQiPing1 OtherActor
          (:then
            (bind _output_get (Variables|Default|SetIsyiqueping true)))
          (:CastFailed
            (Utilities|Casting|CastTofuzhiBP_FireYangQiPing1 OtherActor)
            (bind _output_get_2 (Variables|Default|SetIsyangqiping true))))
        (if (and _output_get _output_get_2)
          (Variables|/Game/BluePrint/FireGameMode.FireGameMode_C|SetIspingziGUIHUAN _asfire_game_mode true)
          (Default|CheckClear (Variables|Default|GetDHZYcollec)))))
    (:CastFailed
      (bind _asbp_zong_he_game_mode (Utilities|Casting|CastToBP_ZongHeGameMode (Game|GetGameMode)))
      (if (Variables|/Game/BluePrint/ZongHeYanLian/BP_ZongHeGameMode.BP_ZongHeGameMode_C|GetzhylIsAfterWork _asbp_zong_he_game_mode)
        (Utilities|Casting|CastTofuzhiBP_FireYangQiPing1 OtherActor
          (:then
            (bind _output_get_3 (Variables|Default|SetIsyiqueping true)))
          (:CastFailed
            (Utilities|Casting|CastTofuzhiBP_FireYangQiPing1 OtherActor)
            (bind _output_get_4 (Variables|Default|SetIsyangqiping true))))
        (if (and _output_get_3 _output_get_4)
          (Variables|/Game/BluePrint/ZongHeYanLian/BP_ZongHeGameMode.BP_ZongHeGameMode_C|SetzhylIspingzizizi _asbp_zong_he_game_mode true)
          (Default|ZhylCheckClear (Variables|Default|Getzhylisclear)))))))

(fn ConstructionScript)