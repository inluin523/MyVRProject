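; BP_GarbagePos is a trigger actor, apparently the target spot for a garbage-clearing task.
; When its Box overlaps a BP_Garbage actor and FireGameMode's IsClearGabarage flag is still false, it hides that garbage's widget and sets the flag.
; After a short delay it hides its own Widget and children.
; The game mode flag makes the completion one-shot.
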(event OnComponentBeginOverlap(Box)
  (params (OverlappedComponent :type Primitive%20Component%20Object%20Reference) (OtherActor :type Actor%20Object%20Reference) (OtherComp :type Primitive%20Component%20Object%20Reference) (OtherBodyIndex :type Integer) (bFromSweep :type Boolean) (SweepResult :type Hit%20Result%20Structure%20%28by%20ref%29))
  (bind _asfire_game_mode (Utilities|Casting|CastToFireGameMode (Game|GetGameMode)))
  (if (not (Variables|/Game/BluePrint/FireGameMode.FireGameMode_C|GetIsClearGabarage _asfire_game_mode))
    (bind _asbp_garbage (Utilities|Casting|CastToBP_Garbage OtherActor))
    (Rendering|SetVisibility (Variables|/Game/ceTest/BP_Garbage.BP_Garbage_C|GetWidget _asbp_garbage) false false)
    (Variables|/Game/BluePrint/FireGameMode.FireGameMode_C|SetIsClearGabarage _asfire_game_mode true)
    (Utilities|FlowControl|Delay 3.0)
    (Rendering|SetVisibility (Variables|Default|GetWidget) false true)))

(event EventBeginPlay)

(event Collision|EventActorBeginOverlap
  (params (OtherActor :type Actor%20Object%20Reference)))

(event EventTick
  (params (DeltaSeconds :type Float%20%28single-precision%29)))

(fn ConstructionScript)